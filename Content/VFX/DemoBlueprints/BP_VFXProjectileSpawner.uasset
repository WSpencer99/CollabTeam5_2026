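; BP_VFXProjectileSpawner is a demo actor that automatically fires BP_VFXProjectile actors from its Arrow component, driven by a WeaponStats struct.
; A looping timer at the fire rate spawns each projectile, passes it the stats and deducts ammo.
; When ammo runs out, a cooldown flag pauses firing and prints a reload message until a reload timer refills the magazine.
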(event Custom|Cooldown
  (bind _weaponstats (Variables|Default|GetWeaponStats))
  (Variables|Default|SetCooldown? false)
  (Utilities|Struct|SetmembersinStruct_WeaponStats _weaponstats (.AmmoCapacity (Utilities|Struct|BreakStruct_WeaponStats _weaponstats))))

(event Custom|Spawn
  (bind _weaponstats (Variables|Default|GetWeaponStats))
  (bind _arrow (Variables|Default|GetArrow))
  (bind (_currentammo _bulletsshot) (Utilities|Struct|BreakStruct_WeaponStats _weaponstats))
  (bind _returnvalue (Transformation|GetWorldTransform _arrow))
  (if (not (Variables|Default|GetCooldown?))
    (bind _returnvalue_2 (Game|SpawnActorfromClass :Class "/Game/VFX/DemoBlueprints/Projectiles/BP_VFXProjectile.BP_VFXProjectile_C" :SpawnTransform (Math|Transform|MakeTransform (.location _returnvalue) (.rotation _returnvalue) "1.000000,1.000000,1.000000") :CollisionHandlingOverride "Undefined" :TransformScaleMethod "MultiplyWithRoot" :Instigator 0))
    (Variables|/Game/VFX/DemoBlueprints/Projectiles/BP_VFXProjectile.BP_VFXProjectile_C|SetBulletStats _returnvalue_2 _weaponstats)
    (Utilities|Struct|SetmembersinStruct_WeaponStats (Variables|Default|GetWeaponStats) (- _currentammo _bulletsshot))
    (if (<= _currentammo 0)
      (Variables|Default|SetCooldown? true)
      (Development|PrintString (Utilities|String|Append (Utilities|GetDisplayName self) " is Reloading"))
      (Utilities|Time|SetTimerbyEvent (delegate Custom|Cooldown) (Utilities|Struct|BreakStruct_WeaponStats (Variables|Default|GetWeaponStats))))))

(event EventBeginPlay
  (bind _weaponstats (Variables|Default|GetWeaponStats))
  (bind (_firerate _ammocapacity) (Utilities|Struct|BreakStruct_WeaponStats _weaponstats))
  (Utilities|Time|SetTimerbyEvent (delegate Custom|Spawn) _firerate true)
  (Utilities|Struct|SetmembersinStruct_WeaponStats _weaponstats _ammocapacity))

(fn ConstructionScript)