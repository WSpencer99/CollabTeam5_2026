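; Pooled projectile that damages actors other than its owner and applies ice, poison or fire status to non-invincible characters.
; On init, player ID sets material, movement type picks mesh, and damage scales size, collision and Niagara trail and aura.
; EnableActor launches it with a lifetime timer; disabling hides it and returns it to its pool location.
; Overlaps spawn a once-per-activation impact; all but piercing shots then disable.
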(event OnComponentBeginOverlap(SphereColl)
  (params (OverlappedComponent :type Primitive%20Component%20Object%20Reference) (OtherActor :type Actor%20Object%20Reference) (OtherComp :type Primitive%20Component%20Object%20Reference) (OtherBodyIndex :type Integer) (bFromSweep :type Boolean) (SweepResult :type Hit%20Result%20Structure%20%28by%20ref%29))
  (bind _returnvalue (Actor|GetComponentbyClass OtherActor "/Game/Tech/Blueprints/Components/StatusFX/BPC_StatusFire.BPC_StatusFire_C"))
  (bind _returnvalue_2 (Actor|GetComponentbyClass OtherActor "/Game/Tech/Blueprints/Components/StatusFX/BPC_StatusIce.BPC_StatusIce_C"))
  (bind _returnvalue_3 (Actor|GetComponentbyClass OtherActor "/Game/Tech/Blueprints/Components/StatusFX/BPC_StatusPoison.BPC_StatusPoison_C"))
  (if (not (== OtherActor (Components|GetOwner)))
    (Variables|Default|SetVFXLoc (Transformation|GetActorLocation))
    (CallFunction|SpawnImpact)
    (Game|Damage|ApplyDamage OtherActor (Variables|Default|GetDamage) 0 (Components|GetOwner))
    (Utilities|FlowControl|Sequence
      (:then_0
        (Audio|PlaySoundatLocation (Variables|Default|GetHitSFX) (Transformation|GetActorLocation) "0, 0, 0" 1.0 1.0 0.0 0 0 0 0)
        (switch Utilities|FlowControl|Switch|SwitchonEnum_ProjectileMovementType (Variables|Default|GetMovementType)
          (:NewEnumerator0
            (Development|PrintString "Default")
            (CallFunction|DisableActor)
            (Collision|SetCollisionResponsetoChannel (Variables|Default|GetSphereColl) "ECC_WorldStatic" "ECR_Overlap")
            (Variables|/Script/Engine.ProjectileMovementComponent|SetbShouldBounce (Variables|Default|GetProjectileMovement) false))
          (:NewEnumerator1
            (Development|PrintString "Bounce")
            (CallFunction|DisableActor)
            (Collision|SetCollisionResponsetoChannel (Variables|Default|GetSphereColl) "ECC_WorldStatic" "ECR_Block")
            (Variables|/Script/Engine.ProjectileMovementComponent|SetbShouldBounce (Variables|Default|GetProjectileMovement) true))
          (:NewEnumerator2
            (Development|PrintString "Pierce"))))
      (:then_1
        (Utilities|IsValid OtherActor
          (:Is%20Valid
            (if (Utilities|ClassIsChildOf (Utilities|GetClass OtherActor) "/Game/Tech/Blueprints/Player/BP_BaseCharacter.BP_BaseCharacter_C")
              (if (not (Variables|/Game/Tech/Blueprints/Components/BPC_HealthComponent.BPC_HealthComponent_C|GetisInvincible (Actor|GetComponentbyClass OtherActor "/Game/Tech/Blueprints/Components/BPC_HealthComponent.BPC_HealthComponent_C")))
                (switch Utilities|FlowControl|Switch|SwitchonEnum_DamageType (Variables|Default|GetDamageType)
                  (:NewEnumerator1
                    (Utilities|IsValid _returnvalue_2
                      (:Is%20Valid
                        (Default|SetTimer _returnvalue_2))
                      (:Is%20Not%20Valid
                        (Game|AddComponentbyClass OtherActor "/Game/Tech/Blueprints/Components/StatusFX/BPC_StatusIce.BPC_StatusIce_C" 2.0))))
                  (:NewEnumerator2
                    (Utilities|IsValid _returnvalue_3
                      (:Is%20Valid
                        (Default|SetTimer _returnvalue_3))
                      (:Is%20Not%20Valid
                        (Game|AddComponentbyClass OtherActor "/Game/Tech/Blueprints/Components/StatusFX/BPC_StatusPoison.BPC_StatusPoison_C" 5.0))))
                  (:NewEnumerator3
                    (Utilities|IsValid _returnvalue
                      (:Is%20Valid
                        (Default|SetTimer _returnvalue))
                      (:Is%20Not%20Valid
                        (Game|AddComponentbyClass OtherActor "/Game/Tech/Blueprints/Components/StatusFX/BPC_StatusFire.BPC_StatusFire_C" 2.0)))))))))))))

(event Custom|SetVFX
  (bind _trail (Variables|Default|GetTrail))
  (bind _damage (Variables|Default|GetDamage))
  (bind _aura (Variables|Default|GetAura))
  ;[0.15 0.15 0.15 0.5] VFX
  (if (== (Utilities|Struct|BreakStruct_VFXParams (Variables|Default|GetVFXParams)) "")
    _
    (else
      _))
  (Niagara|SetNiagaraVariable(Float) _trail "TrailLength" (/ (Variables|Default|GetMovementSpeed) 19999.0))
  (Niagara|SetNiagaraVariable(LinearColor) _trail "TrailColour" (Utilities|Struct|BreakStruct_VFXParams (Variables|Default|GetVFXParams)))
  (Niagara|SetNiagaraVariable(Float) _trail "TrailSize" (Variables|Default|GetDamage))
  (Class|NiagaraComponent|SetAsset (Variables|Default|GetAura) (Utilities|Struct|BreakStruct_VFXParams (Variables|Default|GetVFXParams)) true)
  (Niagara|SetNiagaraVariable(Float) _aura "SpawnRadius" _damage)
  (Niagara|SetNiagaraVariable(Float) _aura "SpawnRate" (* _damage 1e+01)))

(event Custom|SetShape
  ;[0.15 0.15 0.15 0.5] SetColours
  (Components|StaticMesh|SetStaticMesh (Variables|Default|GetSphere) (Utilities|Select :Index (Variables|Default|GetMovementType) :NewEnumerator0 "/Game/VFX/DemoBlueprints/Projectiles/RegularProjectile.RegularProjectile" :NewEnumerator1 "/Engine/BasicShapes/Sphere.Sphere" :NewEnumerator2 "/Game/VFX/DemoBlueprints/Projectiles/PierceProjectile.PierceProjectile" :NewEnumerator3 0)))

(event Custom|Remove
  (Actor|DestroyActor))

(event Custom|SpawnImpact
  (Utilities|FlowControl|DoOnce false
    (:Completed
      (Game|SpawnActorfromClass (Variables|Default|GetImpactEffect) (Math|Transform|MakeTransform (Variables|Default|GetVFXLoc) (Math|Rotator|MakeRotfromZ (Math|Vector|NegateVector (Transformation|GetVelocity))) "1.000000,1.000000,1.000000") "Undefined" "MultiplyWithRoot" 0 (Utilities|Struct|BreakStruct_VFXParams (Variables|Default|GetVFXParams)) 0))))

(event Custom|ResetImpactDoOnce
  (Utilities|FlowControl|DoOnce false) ; enters at Reset
)

(event Custom|SetScale
  (bind _sphere (Variables|Default|GetSphere))
  (bind _damage (Variables|Default|GetDamage))
  (bind _spherecoll (Variables|Default|GetSphereColl))
  (Transformation|SetRelativeScale3D _sphere (Math|Vector|ClampVectorSize (* (Variables|/Script/Engine.SceneComponent|GetRelativeScale3D _sphere) _damage) 0.4 1e+04))
  (Components|Sphere|SetSphereRadius _spherecoll (Math|Float|Clamp(Float) (* (Variables|/Script/Engine.SphereComponent|GetSphereRadius _spherecoll) _damage) 0.4 1e+04) true))

(event Custom|SetSpeed
  (bind _projectilemovement (Variables|Default|GetProjectileMovement))
  (bind _movementspeed (Variables|Default|GetMovementSpeed))
  (Variables|/Script/Engine.ProjectileMovementComponent|SetMaxSpeed _projectilemovement _movementspeed)
  (Variables|/Script/Engine.ProjectileMovementComponent|SetInitialSpeed _projectilemovement _movementspeed))

(event Custom|Init
  (Rendering|Material|SetMaterial (Variables|Default|GetSphere) 0 (Utilities|Select :Index (Variables|Default|GetID) :Option%200 "/Game/VFX/Assets/Materials/MI_BulletP1.MI_BulletP1" :Option%201 "/Game/VFX/Assets/Materials/MI_BulletP2.MI_BulletP2" :Option%202 "/Game/VFX/Assets/Materials/MI_BulletP3.MI_BulletP3" :Option%203 "/Game/VFX/Assets/Materials/MI_BulletP4.MI_BulletP4"))
  (Variables|Default|SetPoolLocation (Transformation|GetActorLocation))
  (CallFunction|SetShape)
  (CallFunction|SetVFX)
  (CallFunction|SetScale)
  (CallFunction|SetSpeed))

(event Custom|DisableActor
  (bind _projectilemovement (Variables|Default|GetProjectileMovement))
  (Default|CallEDisableActor self false)
  (Components|Activation|Deactivate _projectilemovement)
  (Variables|/Script/Engine.MovementComponent|SetVelocity _projectilemovement "0, 0, 0")
  (Variables|Default|SetIsInUse false)
  (Utilities|Time|ClearandInvalidateTimerbyHandle (Variables|Default|GetLifetimeTimer))
  (Rendering|SetActorHiddenInGame true)
  (Collision|SetActorEnableCollision false)
  (Transformation|SetActorLocation (Variables|Default|GetPoolLocation) false true)
  (Variables|Default|SetCanHitSelf? false)
  (CallFunction|ResetImpactDoOnce))

(event Custom|EnableActor
  (params (Transform :type Transform))
  (bind (_location _rotation) (Math|Transform|BreakTransform Transform))
  (Utilities|Time|SetTimerbyEvent (delegate Custom|EnableCanHitSelf) 0.2)
  (Variables|Default|SetIsInUse true)
  (Utilities|Time|ClearandInvalidateTimerbyHandle (Variables|Default|GetLifetimeTimer))
  (bind _returnvalue (Utilities|Time|SetTimerbyEvent (EventDispatchers|CreateEvent :!event Custom|DisableActor) (Variables|Default|GetLifetime)))
  (Variables|Default|SetLifetimeTimer _returnvalue)
  (Transformation|SetActorTransform (Math|Transform|MakeTransform _location _rotation) false true)
  (Components|Activation|Activate (Variables|Default|GetTrail) true)
  (Components|Activation|Activate (Variables|Default|GetProjectileMovement) true)
  (Variables|/Script/Engine.MovementComponent|SetVelocity (Variables|Default|GetProjectileMovement) (* (Variables|Default|GetMovementSpeed) (Math|Vector|GetForwardVector _rotation)))
  (Rendering|SetActorHiddenInGame false)
  (Collision|SetActorEnableCollision true))

(event Custom|ForceDisable
  (bind _projectilemovement (Variables|Default|GetProjectileMovement))
  (Default|CallEDisableActor self true)
  (Components|Activation|Deactivate _projectilemovement)
  (Variables|/Script/Engine.MovementComponent|SetVelocity _projectilemovement "0, 0, 0")
  (Variables|Default|SetIsInUse false)
  (Utilities|Time|ClearandInvalidateTimerbyHandle (Variables|Default|GetLifetimeTimer))
  (Rendering|SetActorHiddenInGame true)
  (Collision|SetActorEnableCollision false)
  (Transformation|SetActorLocation (Variables|Default|GetPoolLocation) false true)
  (Variables|Default|SetCanHitSelf? false)
  (CallFunction|ResetImpactDoOnce))

(event Custom|EnableCanHitSelf
  (Variables|Default|SetCanHitSelf? true))

(event Custom|Destroy
  (Utilities|Time|SetTimerbyEvent (delegate Custom|Remove) (Variables|Default|GetLifetime)))

(event EventBeginPlay
  (Rendering|Material|SetMaterial (Variables|Default|GetSphere) 0 (Utilities|Select :Index (Variables|Default|GetID) :Option%200 "/Game/VFX/Assets/Materials/MI_BulletP1.MI_BulletP1" :Option%201 "/Game/VFX/Assets/Materials/MI_BulletP2.MI_BulletP2" :Option%202 "/Game/VFX/Assets/Materials/MI_BulletP3.MI_BulletP3" :Option%203 "/Game/VFX/Assets/Materials/MI_BulletP4.MI_BulletP4"))
  (Variables|Default|SetPoolLocation (Transformation|GetActorLocation))
  (CallFunction|SetShape)
  (CallFunction|SetVFX)
  (CallFunction|SetScale)
  (CallFunction|SetSpeed))

(event EventDestroyed
  (Development|PrintString (Utilities|GetDisplayName self)))

(fn ConstructionScript)