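; Temporary demo component that derives projectile VFX parameters from a damage type enum, covering None, Ice, Poison and Fire.
; SetParams first runs SetColours, which selects a trail colour and a bullet Niagara system as the aura, with no aura for None.
; It then runs SetVFXStruct, which packs both with impact type, damage and speed into VFXStruct.
; Impact type, damage and speed are only read here, not computed.
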(event Custom|SetVFXStruct
  (Variables|Default|SetVFXStruct (Utilities|Struct|MakeStruct_VFXParams (Variables|Default|GetTrailColour) (Variables|Default|GetImpactType) (Variables|Default|GetAuraType) (Variables|Default|GetDamage) (Variables|Default|GetSpeed))))

(event Custom|SetColours
  (bind _enumdamage (Variables|Default|GetEnumDamage))
  (Variables|Default|SetTrailColour (Utilities|Select :Index _enumdamage :NewEnumerator0 "(R=1.000000,G=1.000000,B=1.000000,A=1.000000)" :NewEnumerator1 "(R=0.000000,G=1.000000,B=1.000000,A=1.000000)" :NewEnumerator2 "(R=0.000000,G=1.000000,B=0.000000,A=1.000000)" :NewEnumerator3 "(R=1.000000,G=0.000000,B=0.000000,A=1.000000)"))
  (Variables|Default|SetAuraType (Utilities|Select :Index _enumdamage :NewEnumerator0 0 :NewEnumerator1 "/Game/VFX/Bullet/Aura/NS_IceBullet.NS_IceBullet" :NewEnumerator2 "/Game/VFX/Bullet/Aura/NS_PoisonBullet.NS_PoisonBullet" :NewEnumerator3 "/Game/VFX/Bullet/Aura/NS_FireBullet.NS_FireBullet")))

(event Custom|SetParams
  (CallFunction|SetColours)
  (CallFunction|SetVFXStruct))