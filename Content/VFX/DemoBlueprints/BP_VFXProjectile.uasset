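; VFX demo projectile that plays an impact effect and removes itself when its collision sphere begins an overlap.
; The overlap spawns the NS_Impact1 Niagara system at the actor's location, with its Z axis opposing the velocity.
; It then deactivates its own Niagara component, hides Sphere and disables that component's collision, and destroys the actor after a short delay.
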(event OnComponentBeginOverlap(SphereColl)
  (params (OverlappedComponent :type Primitive%20Component%20Object%20Reference) (OtherActor :type Actor%20Object%20Reference) (OtherComp :type Primitive%20Component%20Object%20Reference) (OtherBodyIndex :type Integer) (bFromSweep :type Boolean) (SweepResult :type Hit%20Result%20Structure%20%28by%20ref%29))
  (bind _sphere (Variables|Default|GetSphere))
  (Niagara|SpawnSystematLocation "/Game/VFX/Bullet/Impact/NS_Impact1.NS_Impact1" (Transformation|GetActorLocation) (Math|Rotator|MakeRotfromZ (Math|Vector|NegateVector (Transformation|GetVelocity))))
  (Components|Activation|Deactivate (Variables|Default|GetNiagara))
  (Collision|SetCollisionEnabled _sphere "NoCollision")
  (Rendering|SetVisibility _sphere false false)
  (Utilities|FlowControl|Delay 1.0)
  (Actor|DestroyActor))

(event EventBeginPlay)

(fn ConstructionScript)