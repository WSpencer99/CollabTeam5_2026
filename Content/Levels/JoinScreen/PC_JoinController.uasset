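; Player controller for the Join Screen level that lets the player back out to the main menu.
; Releasing Backspace or the gamepad right face button, both bound as debug keys, shows a star-shaped transition widget and starts a matching timer that opens L_MainMenu.
; BeginPlay only prints a test string; the Enhanced Input setup for IMC_Join, its subsystem retry loop and the CallEBackButton call are unconnected.
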(event Custom|ChangeLevel
  (Game|OpenLevel(byObjectReference) "/Game/Levels/MainMenu/L_MainMenu.L_MainMenu"))

(event EventBeginPlay
  (Development|PrintString "Hello"))

(event Input|GamepadEvents|DebugKeyGamepadFaceButtonRight
  (params (Key :type Key%20Structure :default "None") (ActionValue :type Input%20Action%20Value%20Structure))
  (:Released
    (bind _returnvalue (UserInterface|CreateWidget "/Game/UI/Transitions/WBP_TransitionScreen.WBP_TransitionScreen_C" 0 2.0 false true "/Game/UI/Transitions/Images/Star_Transition.Star_Transition"))
    (UserInterface|Viewport|AddtoViewport _returnvalue 97)
    (Utilities|Time|SetTimerbyEvent (delegate Custom|ChangeLevel) 2.0)))

(event Input|KeyboardEvents|DebugKeyBackspace
  (params (Key :type Key%20Structure :default "None") (ActionValue :type Input%20Action%20Value%20Structure))
  (:Released
    (bind _returnvalue (UserInterface|CreateWidget "/Game/UI/Transitions/WBP_TransitionScreen.WBP_TransitionScreen_C" 0 2.0 false true "/Game/UI/Transitions/Images/Star_Transition.Star_Transition"))
    (UserInterface|Viewport|AddtoViewport _returnvalue 97)
    (Utilities|Time|SetTimerbyEvent (delegate Custom|ChangeLevel) 2.0)))

(fn ConstructionScript)