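; BP_Cage is a cage hazard whose static mesh drops a long way down when its Move event is called.
; Move plays the TL_Move timeline, which sets the mesh's relative location each update, using one track for descent and another for a small Y offset.
; The descent track also drives the outer vector lerp, so it scales the Y offset and applies twice to Z.
; A player camera shake node exists but never runs.
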(event Custom|Move
  (bind (_direction _newtrack_0 _newtrack_1) (Timeline|TL_Move Play)
    (:Update
      (Transformation|SetRelativeLocation (Variables|Default|GetStaticMesh) (Math|Vector|Lerp(Vector) (Math|Vector|MakeVector 0.0 0.0 0.0) (Math|Vector|MakeVector 0.0 (Math|Float|Lerp 0.0 2e+01 _newtrack_1) (Math|Float|Lerp 0.0 -1.87e+03 _newtrack_0)) _newtrack_0) false false))))

(event EventBeginPlay)

(event Collision|EventActorBeginOverlap
  (params (OtherActor :type Actor%20Object%20Reference)))

(event EventTick
  (params (DeltaSeconds :type Float%20%28single-precision%29)))

(fn ConstructionScript)