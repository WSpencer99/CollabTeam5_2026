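; BP_ImpactPoison is an impact actor that deals repeated damage to actors inside its area.
; On BeginPlay it calls the parent logic, then starts a short looping timer.
; Each tick of that timer applies BaseDamage to every actor overlapping the Sphere and prints each actor's name on screen.
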(event Custom|DamageTrace
  (for _array_element (Collision|GetOverlappingActors (Variables|Default|GetSphere) 0 :!class /Script/Engine.PrimitiveComponent)
    (Game|Damage|ApplyDamage _array_element (Variables|Default|GetBase%20Damage) 0 0)
    (Development|PrintString (Utilities|GetDisplayName _array_element))))

(event EventBeginPlay
  (|CallParentFunction)
  (Utilities|Time|SetTimerbyEvent (delegate Custom|DamageTrace) 0.2 true))

(fn ConstructionScript
  (|CallParentFunction))