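; BP_ImpactIce is an ice impact actor that slows characters inside its sphere.
; A looping 0.2-second timer finds overlapping actors with a CharacterMovementComponent, saves their current MaxWalkSpeed to InitialMax and cuts it to a tenth.
; End overlap writes InitialMax back.
; InitialMax is one variable shared by all targets and re-read each tick, so slows compound and the restored value can differ from the original speed.
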(event OnComponentEndOverlap(Sphere)
  (params (OverlappedComponent :type Primitive%20Component%20Object%20Reference) (OtherActor :type Actor%20Object%20Reference) (OtherComp :type Primitive%20Component%20Object%20Reference) (OtherBodyIndex :type Integer))
  (bind _returnvalue (Actor|GetComponentbyClass OtherActor "/Script/Engine.CharacterMovementComponent"))
  (Utilities|IsValid _returnvalue
    (:Is%20Valid
      (Variables|/Script/Engine.CharacterMovementComponent|SetMaxWalkSpeed _returnvalue (Variables|Default|GetInitialMax)))))

(event Custom|SlowTrace
  (for _array_element (Collision|GetOverlappingActors (Variables|Default|GetSphere) 0 :!class /Script/Engine.PrimitiveComponent)
    (Utilities|IsValid (Actor|GetComponentbyClass _array_element "/Script/Engine.CharacterMovementComponent")
      (:Is%20Valid
        (bind _output_get (Variables|Default|SetInitialMax (Variables|/Script/Engine.CharacterMovementComponent|GetMaxWalkSpeed (Actor|GetComponentbyClass _array_element "/Script/Engine.CharacterMovementComponent"))))
        (Variables|/Script/Engine.CharacterMovementComponent|SetMaxWalkSpeed (Actor|GetComponentbyClass _array_element "/Script/Engine.CharacterMovementComponent") (* _output_get 0.1))))))

(event EventBeginPlay
  (|CallParentFunction)
  (Utilities|Time|SetTimerbyEvent (delegate Custom|SlowTrace) 0.2 true))

(fn ConstructionScript
  (|CallParentFunction))