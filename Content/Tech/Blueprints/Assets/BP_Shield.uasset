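; BP_Shield is a temporary shield actor that makes its owner invincible for a set duration.
; On BeginPlay it enables the owner's block message, sets the health component's IsInvincible and scales up its sphere via a timeline.
; A timer then fades the dynamic material's opacity, restores vulnerability and the block toggle, and destroys the actor.
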(event Custom|DestroySelf
  (bind _returnvalue (Components|GetOwner))
  (bind _opacity (Timeline|Timeline_0 Play)
    (:Update
      (Rendering|Material|SetScalarParameterValue (Variables|Default|GetShieldMat) "Opacity" _opacity :!class /Script/Engine.MaterialInstanceDynamic))
    (:Finished
      (Variables|/Game/Tech/Blueprints/Components/BPC_HealthComponent.BPC_HealthComponent_C|SetisInvincible (Actor|GetComponentbyClass _returnvalue "/Game/Tech/Blueprints/Components/BPC_HealthComponent.BPC_HealthComponent_C") false)
      (Class|BPIPlayer|IToggleBlock(Message) _returnvalue false)
      (Actor|DestroyActor))))

(event EventBeginPlay
  (Class|BPIPlayer|IToggleBlock(Message) (Components|GetOwner) true)
  (Utilities|Time|SetTimerbyEvent (delegate Custom|DestroySelf) (Variables|Default|GetShieldDuration))
  (Variables|/Game/Tech/Blueprints/Components/BPC_HealthComponent.BPC_HealthComponent_C|SetisInvincible (Actor|GetComponentbyClass (Components|GetOwner) "/Game/Tech/Blueprints/Components/BPC_HealthComponent.BPC_HealthComponent_C") true)
  (bind _scale (Timeline|Timeline Play)
    (:Update
      (Transformation|SetWorldScale3D (Variables|Default|GetSphere) _scale))))

(fn ConstructionScript
  (bind _returnvalue (Rendering|Material|CreateDynamicMaterialInstance (Variables|Default|GetSphere) 0 "/Game/VFX/Assets/Materials/M_Shield.M_Shield" "None" :!class /Script/Engine.PrimitiveComponent))
  (Variables|Default|SetShieldMat _returnvalue))