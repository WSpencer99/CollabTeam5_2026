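; BP_Projectile is a reusable projectile actor that toggles between active and hidden states instead of being destroyed, which suggests object pooling.
; Activate unhides it, launches it along the Sphere's forward vector at Speed and starts a lifetime timer.
; A hit on anything but its owner applies fixed damage; that hit or timer expiry calls Deactivate, which hides it, stops movement and clears IsActive.
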(event Custom|StartDeleteTimer
  ;[0.15 0.15 0.15 0.5] Projectile Lifetime
  (Utilities|Time|SetTimerbyEvent (delegate Custom|Delete) (Variables|Default|GetLifetime)))

(event Custom|Delete
  ;[0.15 0.15 0.15 0.5] Projectile Lifetime
  (CallFunction|Deactivate))

(event Collision|EventHit
  (params (MyComp :type Primitive%20Component%20Object%20Reference) (Other :type Actor%20Object%20Reference) (OtherComp :type Primitive%20Component%20Object%20Reference) (bSelfMoved :type Boolean) (HitLocation :type Vector :default "0, 0, 0") (HitNormal :type Vector :default "0, 0, 0") (NormalImpulse :type Vector :default "0, 0, 0") (Hit :type Hit%20Result%20Structure%20%28by%20ref%29))
  (if (not (== Other (Components|GetOwner)))
    (Development|PrintString "Hello")
    (Game|Damage|ApplyDamage Other 1e+01 0 0)
    (CallFunction|Deactivate)))

(fn ConstructionScript)

(fn Activate
  (bind _projectilemovement (Variables|Default|GetProjectileMovement))
  (Development|PrintString "Fire")
  (Rendering|SetActorHiddenInGame false)
  (Components|Activation|Activate _projectilemovement true)
  (Variables|/Script/Engine.MovementComponent|SetVelocity _projectilemovement (* (Math|Vector|GetForwardVector (Variables|Default|GetSphere)) (Variables|Default|GetSpeed)))
  (CallFunction|StartDeleteTimer))

(fn Deactivate
  (Development|PrintString "collect")
  (Rendering|SetActorHiddenInGame true)
  (Components|Activation|Deactivate (Variables|Default|GetProjectileMovement))
  (Variables|Default|SetIsActive false))