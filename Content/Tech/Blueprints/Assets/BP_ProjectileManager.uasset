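; BP_ProjectileManager is an object pool that pre-spawns BP_Projectile actors and hands them out for reuse.
; On BeginPlay it spawns projectiles at PoolLocation based on PoolSize, gives each a reference back to itself, deactivates it and stores it in ProjectilePool.
; GetProjectile linearly searches the pool for the first inactive projectile, flags it active and returns it, with no growth when all are in use.
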(event EventBeginPlay
  (for _index (range 0 (Variables|Default|GetPoolSize))
    (bind _returnvalue (Game|SpawnActorfromClass "/Game/Tech/Blueprints/Assets/BP_Projectile.BP_Projectile_C" (Variables|Default|GetPoolLocation) "Undefined" "MultiplyWithRoot" 0 0))
    (Variables|/Game/Tech/Blueprints/Assets/BP_Projectile.BP_Projectile_C|SetPoolManager _returnvalue self)
    (Default|Deactivate _returnvalue)
    (Utilities|Array|Add (Variables|Default|GetProjectilePool) _returnvalue)))

(fn ConstructionScript)

(fn GetProjectile
  (for _array_element (Variables|Default|GetProjectilePool)
    (if (not (Variables|/Game/Tech/Blueprints/Assets/BP_Projectile.BP_Projectile_C|GetIsActive _array_element))
      (Variables|/Game/Tech/Blueprints/Assets/BP_Projectile.BP_Projectile_C|SetIsActive _array_element true)
      (return _array_element))))