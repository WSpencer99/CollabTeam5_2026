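; BP_PickupSpawner spawns random pickup classes from an array at the positions of randomly chosen spawn location actors.
; BeginPlay sets a looping timer, with an interval randomized once between min and max spawn times, and calls SpawnPickup.
; SpawnPickup spawns the actor and prints debug text, including a location index from a separate random pick that may differ from the one used.
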(event Custom|SpawnPickup
  (bind _spawnlocations (Variables|Default|GetSpawnLocations))
  (bind (_outitem _outindex) (Utilities|Array|Random _spawnlocations))
  ;[0.4793 0.000304 0.8308 0.502] Pickup Spawn
  (Game|SpawnActorfromClass (.OutItem (Utilities|Array|Random (Variables|Default|GetPickupArray))) (Math|Transform|MakeTransform (Transformation|GetActorLocation _outitem) "0, 0, 0" "1.000000,1.000000,1.000000") "Undefined" "MultiplyWithRoot" 0 0)
  (Development|PrintString "SPAWNED" true true "(R=1.000000,G=0.863157,B=0.000000,A=1.000000)")
  (Development|PrintString (Utilities|String|ToString(Integer) _outindex) true true "(R=1.000000,G=0.000000,B=0.109359,A=1.000000)"))

(event EventBeginPlay
  ;[0.4793 0.000304 0.8308 0.502] Spawn Timer
  (Utilities|Time|SetTimerbyEvent (EventDispatchers|CreateEvent :!event Custom|SpawnPickup) (Math|Random|RandomFloatinRange (Variables|Default|GetMinSpawnTime) (Variables|Default|GetMaxSpawnTime)) true)
  (CallFunction|SpawnPickup))

(fn ConstructionScript)