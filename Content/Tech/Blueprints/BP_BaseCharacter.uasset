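; Base player character for a side-on shooter that moves along the world Y axis, jumps and fires projectiles through Enhanced Input.
; Stick aim beyond a deadzone pitches AimArm via Atan2 and flips the Cylinder when aiming backwards.
; Fire spawns BP_Base_Projectile at the ArrowFire transform.
; An uncalled AimLocation helper attempts to project a point onto the actor's X plane, but its Z term divides by zero.
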(event Input|EnhancedActionEvents|EnhancedInputActionIA_Fire
  (params (ActionValue :type Boolean) (ElapsedSeconds :type Float%20%28double-precision%29) (TriggeredSeconds :type Float%20%28double-precision%29) (InputAction :type Input%20Action%20Object%20Reference :default "/Game/Tech/Input/IA_Fire.IA_Fire"))
  (bind _arrowfire (Variables|Default|GetArrowFire))
  ;[0.15 0.15 0.15 0.5] Basic Firing
  (:Started
    (Development|PrintString "Hello")
    (Game|SpawnActorfromClass "/Game/Tech/Blueprints/BP_Base_Projectile.BP_Base_Projectile_C" (Math|Transform|MakeTransform (Transformation|GetWorldLocation _arrowfire) (Transformation|GetWorldRotation _arrowfire) "1.000000,1.000000,1.000000") "Undefined" "MultiplyWithRoot" 0 0)))

(event Input|EnhancedActionEvents|EnhancedInputActionIA_Move
  (params (ActionValue :type Float%20%28double-precision%29) (ElapsedSeconds :type Float%20%28double-precision%29) (TriggeredSeconds :type Float%20%28double-precision%29) (InputAction :type Input%20Action%20Object%20Reference :default "/Game/Tech/Input/IA_Move.IA_Move"))
  ;[0.15 0.15 0.15 0.5] Input
  (Pawn|Input|AddMovementInput (Math|Vector|MakeVector 0.0 ActionValue 0.0) 1.0 false)
  (if (> ActionValue 0.0)
    _))

(event Input|EnhancedActionEvents|EnhancedInputActionIA_Jump
  (params (ActionValue :type Boolean) (ElapsedSeconds :type Float%20%28double-precision%29) (TriggeredSeconds :type Float%20%28double-precision%29) (InputAction :type Input%20Action%20Object%20Reference :default "/Game/Tech/Input/IA_Jump.IA_Jump"))
  ;[0.15 0.15 0.15 0.5] Input
  (Character|Jump))

(event Input|EnhancedActionEvents|EnhancedInputActionIA_Aim
  (params (ActionValue :type Vector%202D%20Structure) (ElapsedSeconds :type Float%20%28double-precision%29) (TriggeredSeconds :type Float%20%28double-precision%29) (InputAction :type Input%20Action%20Object%20Reference :default "/Game/Tech/Input/IA_Aim.IA_Aim"))
  (bind _returnvalue (* (.y ActionValue) -1.0))
  (bind _cylinder (Variables|Default|GetCylinder))
  (bind _returnvalue_2 (Math|Trig|Atan2(Radians) _returnvalue (.x ActionValue)))
  (bind _returnvalue_3 (Math|Trig|RadiansToDegrees _returnvalue_2))
  ;[0.15 0.15 0.15 0.5] Aiming -
  (if (> (Math|Float|Absolute(Float) (Math|Vector2D|Vector2DLength (Math|Vector2D|MakeVector2D (.x ActionValue) (.y ActionValue)))) (Variables|Default|Getdeadzone))
    (Transformation|SetRelativeRotation (Variables|Default|GetAimArm) (Math|Rotator|MakeRotator 0.0 _returnvalue_3 0.0) false false)
    (if (> (Math|Float|Absolute(Float) _returnvalue_3) 9e+01)
      (Transformation|SetRelativeRotation _cylinder (Math|Rotator|MakeRotator 0.0 0.0 1.8e+02) false false)
      (else
        (Transformation|SetRelativeRotation _cylinder (Math|Rotator|MakeRotator 0.0 0.0 0.0) false false)))))

(event EventBeginPlay
  ;[0.15 0.15 0.15 0.5] Setup Input
  (Input|AddMappingContext (PlayerController|LocalPlayerSubsystems|GetEnhancedInputLocalPlayerSubsystem (Game|GetPlayerController 0)) "/Game/Tech/Input/IMC_Player.IMC_Player" 0 "(bIgnoreAllPressedKeysUntilRelease=True,bForceImmediately=False,bNotifyUserSettings=False)"))

(fn ConstructionScript)

(fn AimLocation
  (params (InputLocation :type Vector) (InputPin :type Vector))
  (bind (_x _y _z) (Math|Vector|BreakVector InputLocation))
  (bind (_x_2 _y_2) (Math|Vector|BreakVector InputPin))
  (bind _returnvalue (Transformation|GetActorLocation))
  (return (Math|Vector|MakeVector _x (+ (/ (* (- (.x _returnvalue) _x) (- _y_2 _y)) (- _x_2 _x)) _y) (+ _z (/ (* (- (.x _returnvalue) _x) (- _z _z)) (- _x _x))))))