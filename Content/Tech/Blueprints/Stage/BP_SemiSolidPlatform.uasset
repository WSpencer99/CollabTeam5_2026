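; BP_SemiSolidPlatform is a stage platform that characters pass up through from below and can drop through from above.
; Overlapping the Under volume disables collision on the Cube for BP_BaseCharacter actors, and leaving restores it.
; Entering the Above volume disables collision only if the character's Fall flag is set, otherwise enables it, and exiting re-enables it.
; Collision toggles on the whole Cube rather than per character, and the drop-through branch prints a debug string.
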(event OnComponentBeginOverlap(Under)
  (params (OverlappedComponent :type Primitive%20Component%20Object%20Reference) (OtherActor :type Actor%20Object%20Reference) (OtherComp :type Primitive%20Component%20Object%20Reference) (OtherBodyIndex :type Integer) (bFromSweep :type Boolean) (SweepResult :type Hit%20Result%20Structure%20%28by%20ref%29))
  (Utilities|Casting|CastToBP_BaseCharacter OtherActor)
  (Collision|SetCollisionEnabled (Variables|Default|GetCube) "NoCollision"))

(event OnComponentEndOverlap(Under)
  (params (OverlappedComponent :type Primitive%20Component%20Object%20Reference) (OtherActor :type Actor%20Object%20Reference) (OtherComp :type Primitive%20Component%20Object%20Reference) (OtherBodyIndex :type Integer))
  (Utilities|Casting|CastToBP_BaseCharacter OtherActor)
  (Collision|SetCollisionEnabled (Variables|Default|GetCube) "QueryAndPhysics"))

(event OnComponentBeginOverlap(Above)
  (params (OverlappedComponent :type Primitive%20Component%20Object%20Reference) (OtherActor :type Actor%20Object%20Reference) (OtherComp :type Primitive%20Component%20Object%20Reference) (OtherBodyIndex :type Integer) (bFromSweep :type Boolean) (SweepResult :type Hit%20Result%20Structure%20%28by%20ref%29))
  (bind _cube (Variables|Default|GetCube))
  (bind _asbp_base_character (Utilities|Casting|CastToBP_BaseCharacter OtherActor))
  (if (Variables|/Game/Tech/Blueprints/Player/BP_BaseCharacter.BP_BaseCharacter_C|GetFall? _asbp_base_character)
    (Collision|SetCollisionEnabled _cube "NoCollision")
    (Development|PrintString "Hello")
    (else
      (Collision|SetCollisionEnabled _cube "QueryAndPhysics"))))

(event OnComponentEndOverlap(Above)
  (params (OverlappedComponent :type Primitive%20Component%20Object%20Reference) (OtherActor :type Actor%20Object%20Reference) (OtherComp :type Primitive%20Component%20Object%20Reference) (OtherBodyIndex :type Integer))
  (Utilities|Casting|CastToBP_BaseCharacter OtherActor)
  (Collision|SetCollisionEnabled (Variables|Default|GetCube) "QueryAndPhysics"))

(fn ConstructionScript)