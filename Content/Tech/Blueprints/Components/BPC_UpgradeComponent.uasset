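; Upgrade component that picks a random positive or negative stat change of a requested rarity, intended to weight bad luck by leaderboard position.
; Upgrade stores the rarity, then PositionCheck rolls polarity against BadLuckChance, though its switch uses a literal first place, fixing that chance.
; GetCorrectUpgrade redraws random UpgradeTable rows, storing StatChange, until rarity and polarity match.
; The match flag is never reset here, and StatChange is not applied.
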(event Custom|Upgrade
  (params (Rarity :type Enum_Rarity%20Enum :default "NewEnumerator0"))
  ;[0.15 0.15 0.15 0.5] Upgrade Sequence
  (Variables|Default|SetSelectedRarity Rarity)
  (CallFunction|PositionCheck)
  (CallFunction|GetCorrectUpgrade))

(event Custom|PositionCheck
  ;[0.15 0.15 0.15 0.5] Checks Player's Current Position
  (switch Utilities|FlowControl|Switch|SwitchonEnum_LeaderBoardPos (Utilities|Enum|LiteralenumEnum_LeaderBoardPos "NewEnumerator0")
    (:NewEnumerator0
      (bind _output_get (Variables|Default|SetBadLuckChance 50)))
    (:NewEnumerator1
      (bind _output_get_2 (Variables|Default|SetBadLuckChance 35)))
    (:NewEnumerator2
      (bind _output_get_3 (Variables|Default|SetBadLuckChance 15)))
    (:NewEnumerator3
      (bind _output_get_4 (Variables|Default|SetBadLuckChance 0))))
  (if (>= (Math|Random|RandomIntegerinRange 0 100) (Utilities|Select :Index (Variables|Default|GetCurrentLeaderboardPos) :Option%200 _output_get :Option%201 _output_get_2 :Option%202 _output_get_3 :Option%203 _output_get_4))
    (Variables|Default|SetPositiveNegative "NewEnumerator0")
    (Variables|Default|SetIsPositiveUpgrade true)
    (else
      (Variables|Default|SetPositiveNegative "NewEnumerator1")
      (Variables|Default|SetIsPositiveUpgrade false))))

(event Custom|GetCorrectUpgrade
  ;[0.15 0.15 0.15 0.5] Gets Upgrade Data
  (while (not (Variables|Default|GetCorrectUpgrade))
    (bind _outrownames (DataTable|GetDataTableRowNames "/Game/Levels/Shop/Upgrades/UpgradeTable.UpgradeTable"))
    (bind _returnvalue (Utilities|GetDataTableRow "/Game/Levels/Shop/Upgrades/UpgradeTable.UpgradeTable" (Utilities|Array|Get(acopy) _outrownames (Math|Random|RandomIntegerinRange 0 (Utilities|Array|Length _outrownames))))
      (:then
        (Variables|Default|SetStat%20Change (.StatChange (Utilities|Struct|Breaks_UpgradeTemplate _returnvalue)))
        (if (Utilities|Enum|Equal(Enum) (Variables|Default|GetSelectedRarity) (.Rarity (Utilities|Struct|Breaks_UpgradeTemplate _returnvalue)))
          (if (== (.Positive (Utilities|Struct|Breaks_UpgradeTemplate _returnvalue)) (Variables|Default|GetIsPositiveUpgrade))
            (Variables|Default|SetCorrectUpgrade true)
            (else
              (Variables|Default|SetCorrectUpgrade false))))))))