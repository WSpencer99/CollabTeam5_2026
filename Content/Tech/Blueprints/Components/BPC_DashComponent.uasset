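; Dash component that launches its owning character along the look direction, or opposite it when wall sliding without aiming.
; FLaunchChar spawns a Niagara burst, plays a montage, zeroes velocity and friction, then applies a velocity-change impulse.
; StopDash restores braking and ground friction but not falling lateral friction, then starts the cooldown to ResetDash.
; Dispatchers announce dash start, completion and recharge, while a Dashing flag blocks re-dashing until reset.
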(event Custom|StopDash
  (bind _returnvalue (Components|GetOwner))
  (bind _returnvalue_2 (Actor|GetComponentbyClass _returnvalue "/Script/Engine.CharacterMovementComponent"))
  (Default|CallEDashComplete)
  (Variables|/Script/Engine.CharacterMovementComponent|SetBrakingFriction _returnvalue_2 2.0)
  (Variables|/Script/Engine.CharacterMovementComponent|SetGroundFriction _returnvalue_2 8.0)
  (Utilities|Time|SetTimerbyEvent (delegate Custom|ResetDash) (Variables|Default|GetDashCooldown)))

(event Custom|ResetDash
  (Variables|Default|SetDashing? false)
  (Default|CallEDashCharged))

(fn FLaunchChar
  (params (LookingAt :type Rotator) (IsWallSliding? :type Boolean) (IsAiming? :type Boolean))
  (bind _returnvalue (Math|Vector|GetForwardVector LookingAt))
  (bind _returnvalue_2 (Components|GetOwner))
  (bind _returnvalue_3 (Actor|GetComponentbyClass _returnvalue_2 "/Script/Engine.CharacterMovementComponent"))
  (if (not (Variables|Default|GetDashing?))
    (Utilities|FlowControl|Sequence
      (:then_0
        (Niagara|SpawnSystematLocation "/Game/VFX/Movement/NS_Dash.NS_Dash" (Transformation|GetActorLocation _returnvalue_2) (select (and (not IsAiming?) IsWallSliding?) (Math|Rotator|MakeRotfromZ (Math|Vector|NegateVector _returnvalue)) (Math|Rotator|MakeRotfromZ _returnvalue)))
        (Class|BPIPlayer|IPlayMontage(Message) (Components|GetOwner) "/Game/Assets/Character/Animations/AM_DashFast_Montage.AM_DashFast_Montage"))
      (:then_1
        (Variables|Default|SetDashing? true)
        (Variables|/Script/Engine.MovementComponent|SetVelocity _returnvalue_3 "0, 0, 0")
        (Variables|/Script/Engine.CharacterMovementComponent|SetFallingLateralFriction _returnvalue_3 0.0)
        (Variables|/Script/Engine.CharacterMovementComponent|SetBrakingFriction _returnvalue_3 0.0)
        (Variables|/Script/Engine.CharacterMovementComponent|SetGroundFriction _returnvalue_3 0.0)
        (Physics|AddImpulse _returnvalue_3 (* (select (and (not IsAiming?) IsWallSliding?) (Math|Vector|NegateVector (Math|Vector|GetForwardVector LookingAt)) (Math|Vector|GetForwardVector LookingAt)) (Variables|Default|GetDashStrength)) true)
        (Default|CallEStartDash)
        (Utilities|Time|SetTimerbyEvent (EventDispatchers|CreateEvent :!event Custom|StopDash) 0.5)))))