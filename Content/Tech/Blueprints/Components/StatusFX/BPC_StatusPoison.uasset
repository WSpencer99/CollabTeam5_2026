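; Poison status-effect component that drains its owner's ammo by a percentage every second for a limited lifetime.
; On BeginPlay, owners with a CharacterMovementComponent get attached poison VFX and sound, a looping interface-driven drain timer and a lifetime timer that removes everything.
; A separate sphere-trace function, not called within this component, applies damage once per unique hit actor.
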(event Custom|DrainAmmo
  (bind _percenttodrain (Variables|Default|GetPercentToDrain))
  (bind _returnvalue (/ _percenttodrain 100))
  (Development|PrintString (Utilities|String|ToString(Float) _returnvalue) true true "(R=1.000000,G=0.927213,B=0.000000,A=1.000000)")
  (Class|BPIPlayer|IDrainAmmo(Message) (Components|GetOwner) _returnvalue))

(event Custom|RemoveSelf
  (Components|DestroyComponent (Variables|Default|GetVFX))
  (Components|DestroyComponent (Variables|Default|GetAudio))
  (Components|DestroyComponent))

(event Custom|SetTimer
  (Utilities|Time|ClearandInvalidateTimerbyHandle (Variables|Default|GetLifetimeTimer))
  (Utilities|Time|SetTimerbyEvent (delegate Custom|RemoveSelf) (Variables|Default|GetLifeTime))
  (Variables|Default|SetLifetimeTimer ""))

(event EventBeginPlay
  (Utilities|IsValid (Actor|GetComponentbyClass (Components|GetOwner) "/Script/Engine.CharacterMovementComponent")
    (:Is%20Valid
      (Utilities|Time|SetTimerbyEvent (delegate Custom|DrainAmmo) 1.0 true)
      (CallFunction|SetTimer)
      (bind _returnvalue (Niagara|SpawnSystemAttached "/Game/VFX/Magic/NS_OnPoison.NS_OnPoison" (Variables|/Script/Engine.Actor|GetRootComponent (Components|GetOwner)) "None" "0, 0, 0" "0, 0, 0" "KeepRelativeOffset" false))
      (Variables|Default|SetVFX _returnvalue)
      (bind _returnvalue_2 (Audio|SpawnSoundAttached "/Game/Sound/SFX/PlayerStates/MS_PoisonStatus.MS_PoisonStatus" (Variables|/Script/Engine.Actor|GetRootComponent (Components|GetOwner)) "None" "0, 0, 0" "0, 0, 0" "SnapToTargetIncludingScale" true 1.0 1.0 0.0 0 0 false))
      (Variables|Default|SetAudio _returnvalue_2))))

(fn FPoisonTrace
  (params (ObjectTypes :type Array%20of%20EObjectTypeQuery%20Enums :default "ObjectTypeQuery1") (End :type Vector) (Start :type Vector))
  (Utilities|FlowControl|Sequence
    (:then_1
      (bind _outhits (Collision|MultiSphereTraceForObjects Start End 2e+02 ObjectTypes false 0 "None" true "(R=1.000000,G=0.000000,B=0.000000,A=1.000000)" "(R=0.000000,G=1.000000,B=0.000000,A=1.000000)" 1.0))
      (for _array_element _outhits
        (if (not (Utilities|Array|ContainsItem (LocalVariables|GetL_DamgedActors) (.HitActor (Collision|BreakHitResult _array_element))))
          (Development|PrintString (Utilities|GetDisplayName (.HitActor (Collision|BreakHitResult _array_element))))
          (Game|Damage|ApplyDamage (.HitActor (Collision|BreakHitResult _array_element)) 1.0 0 0)
          (Utilities|Array|Add (LocalVariables|GetL_DamgedActors) (.HitActor (Collision|BreakHitResult _array_element))))))))