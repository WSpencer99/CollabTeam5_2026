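; Burning status effect component that damages its owner over time, active only when the owner has a CharacterMovementComponent.
; On BeginPlay it reads max health through an interface, attaches fire Niagara and sound, and starts a looping burn timer.
; Damage ticks are scaled to total about a fifth of max health over LifeTime.
; SetTimer restarts the lifetime countdown, whose expiry destroys the effects and the component.
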(event Custom|Burn
  (Game|Damage|ApplyDamage (Components|GetOwner) (/ (/ (stale EventBeginPlay _output_get) (* (Variables|Default|GetLifeTime) 1e+01)) 5.0) 0 0))

(event Custom|RemoveSelf
  (Utilities|IsValid (Variables|Default|GetVFX)
    (:Is%20Valid
      (Components|DestroyComponent (Variables|Default|GetVFX))
      (Components|DestroyComponent (Variables|Default|GetAudio))
      (Components|DestroyComponent))))

(event Custom|SetTimer
  (Utilities|Time|ClearandInvalidateTimerbyHandle (Variables|Default|GetLifetimeTimer))
  (bind _returnvalue (Utilities|Time|SetTimerbyEvent (delegate Custom|RemoveSelf) (Variables|Default|GetLifeTime)))
  (Variables|Default|SetLifetimeTimer _returnvalue))

(event EventBeginPlay
  (bind _returnvalue (Components|GetOwner))
  (Utilities|IsValid (Actor|GetComponentbyClass _returnvalue "/Script/Engine.CharacterMovementComponent")
    (:Is%20Valid
      (bind _maxhealth (Class|BPIPlayer|IGetHealth(Message) _returnvalue))
      (bind _output_get (Variables|Default|SetMax%20Health _maxhealth))
      (Utilities|Time|SetTimerbyEvent (delegate Custom|Burn) 0.1 true)
      (CallFunction|SetTimer)
      (bind _returnvalue_2 (Niagara|SpawnSystemAttached "/Game/VFX/Magic/NS_OnFire.NS_OnFire" (Variables|/Script/Engine.Actor|GetRootComponent (Components|GetOwner)) "None" "0, 0, 0" "0, 0, 0" "KeepRelativeOffset" false))
      (Variables|Default|SetVFX _returnvalue_2)
      (bind _returnvalue_3 (Audio|SpawnSoundAttached "/Game/Sound/SFX/PlayerStates/MS_FireStatus.MS_FireStatus" (Variables|/Script/Engine.Actor|GetRootComponent (Components|GetOwner)) "None" "0, 0, 0" "0, 0, 0" "SnapToTargetIncludingScale" true 1.0 1.0 0.0 0 0 false))
      (Variables|Default|SetAudio _returnvalue_3))))