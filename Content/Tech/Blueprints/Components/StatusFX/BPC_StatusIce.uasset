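; Ice status effect component that slows its owner to a tenth of its max walk speed for a limited lifetime.
; On BeginPlay, if the owner has a CharacterMovementComponent, it caches the speed, starts a timer and attaches ice VFX plus the MS_PoisonStatus sound to the root.
; When the timer fires, it restores the cached speed and destroys the effects and itself.
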(event Custom|RemoveSelf
  (bind _returnvalue (Components|GetOwner))
  (bind _returnvalue_2 (Actor|GetComponentbyClass _returnvalue "/Script/Engine.CharacterMovementComponent"))
  (Utilities|IsValid _returnvalue_2
    (:Is%20Valid
      (Variables|/Script/Engine.CharacterMovementComponent|SetMaxWalkSpeed _returnvalue_2 (Variables|Default|GetInitialMax)))
    (:Is%20Not%20Valid
      _))
  (Components|DestroyComponent (Variables|Default|GetVFX))
  (Components|DestroyComponent (Variables|Default|GetAudio))
  (Components|DestroyComponent))

(event Custom|SetTimer
  (Utilities|Time|ClearandInvalidateTimerbyHandle (Variables|Default|GetLifetimeTimer))
  (Utilities|Time|SetTimerbyEvent (delegate Custom|RemoveSelf) (Variables|Default|GetLifeTime))
  (Variables|Default|SetLifetimeTimer ""))

(event EventBeginPlay
  (bind _returnvalue (Components|GetOwner))
  (bind _returnvalue_2 (Actor|GetComponentbyClass _returnvalue "/Script/Engine.CharacterMovementComponent"))
  (Utilities|IsValid _returnvalue_2
    (:Is%20Valid
      (bind _output_get (Variables|Default|SetInitialMax (Variables|/Script/Engine.CharacterMovementComponent|GetMaxWalkSpeed _returnvalue_2)))
      (Variables|/Script/Engine.CharacterMovementComponent|SetMaxWalkSpeed _returnvalue_2 (* _output_get 0.1))
      (CallFunction|SetTimer)
      (bind _returnvalue_3 (Niagara|SpawnSystemAttached "/Game/VFX/Magic/NS_OnIce.NS_OnIce" (Variables|/Script/Engine.Actor|GetRootComponent (Components|GetOwner)) "None" "0, 0, 0" "0, 0, 0" "KeepRelativeOffset" false))
      (Variables|Default|SetVFX _returnvalue_3)
      (bind _returnvalue_4 (Audio|SpawnSoundAttached "/Game/Sound/SFX/PlayerStates/MS_PoisonStatus.MS_PoisonStatus" (Variables|/Script/Engine.Actor|GetRootComponent (Components|GetOwner)) "None" "0, 0, 0" "0, 0, 0" "SnapToTargetIncludingScale" true 1.0 1.0 0.0 0 0 false))
      (Variables|Default|SetAudio _returnvalue_4))))