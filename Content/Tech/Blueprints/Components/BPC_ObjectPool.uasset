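; Actor component that pools pre-spawned projectiles for a player's weapon, built from its upgraded weapon stats.
; On init it spawns and disables three times the ammo capacity, configuring damage, movement, and damage-type VFX and sound.
; Functions hand out free or specific projectiles and track them in an in-use list, whose first entry serves as the oldest.
; Each projectile's disable event is bound, and removal functions clear entries from that list.
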(event Custom|InitPool
  (bind _weapon_stats (Variables|Default|GetWeapon%20Stats))
  ;[0.15 0.15 0.15 0.5] Initialise
  (bind _output_get (Variables|Default|SetPoolSize (* (.ammocapacity _weapon_stats) 3)))
  (for _index (range 1 _output_get)
    (bind _returnvalue (Game|SpawnActorfromClass (Variables|Default|GetPoolActorClass) (Math|Transform|MakeTransform (Variables|Default|GetPoolDisabledLoc) "0, 0, 0" "1.000000,1.000000,1.000000") "Undefined" "MultiplyWithRoot" (Components|GetOwner) (Utilities|Struct|MakeStruct_VFXParams (Utilities|Select :Index (.damagetype _weapon_stats) :NewEnumerator0 "(R=1.000000,G=1.000000,B=1.000000,A=1.000000)" :NewEnumerator1 "(R=0.000000,G=1.000000,B=1.000000,A=1.000000)" :NewEnumerator2 "(R=0.000000,G=1.000000,B=0.000000,A=1.000000)" :NewEnumerator3 "(R=1.000000,G=0.000000,B=0.000000,A=1.000000)" :NewEnumerator4 "") (Utilities|Select :Index (.damagetype _weapon_stats) :NewEnumerator0 "/Game/VFX/Bullet/Impact/NS_Impact1.NS_Impact1" :NewEnumerator1 "/Game/VFX/Bullet/Impact/NS_Impact1.NS_Impact1" :NewEnumerator2 "/Game/VFX/Bullet/Impact/NS_Impact1.NS_Impact1" :NewEnumerator3 "/Game/VFX/Bullet/Impact/NS_Impact1.NS_Impact1" :NewEnumerator4 0) (Utilities|Select :Index (.damagetype _weapon_stats) :NewEnumerator0 0 :NewEnumerator1 "/Game/VFX/Bullet/Aura/NS_IceBullet.NS_IceBullet" :NewEnumerator2 "/Game/VFX/Bullet/Aura/NS_PoisonBullet.NS_PoisonBullet" :NewEnumerator3 "/Game/VFX/Bullet/Aura/NS_FireBullet.NS_FireBullet" :NewEnumerator4 0) (Math|Float|MapRangeClamped (.damage _weapon_stats) 1e+01 5e+01 1.0 3.0) (.projectilespeed _weapon_stats)) (.damage _weapon_stats) (.movementtype _weapon_stats) (.projectilespeed _weapon_stats) (.damagetype _weapon_stats) (.impactactor _weapon_stats) (Utilities|Select :Index (.damagetype _weapon_stats) :NewEnumerator0 "/Game/Sound/SFX/AmmoTypes/MS_ProjectileHit.MS_ProjectileHit" :NewEnumerator1 "/Game/Sound/SFX/AmmoTypes/MS_IceHit.MS_IceHit" :NewEnumerator2 "/Game/Sound/SFX/AmmoTypes/MS_PoisonHit.MS_PoisonHit" :NewEnumerator3 "/Game/Sound/SFX/AmmoTypes/MS_FireHit.MS_FireHit" :NewEnumerator4 0) (Variables|Default|GetPlayer%20ID) 0))
    (Default|DisableActor _returnvalue)
    (Utilities|Array|Add (Variables|Default|GetObjectPool) _returnvalue)
    (EventDispatchers|BindEventtoEDisableActor _returnvalue (EventDispatchers|CreateEvent :!event Custom|Remove))))

(event Custom|Remove
  (params (Target :type BP%20VFX%20Projectile%20Object%20Reference) (Forced :type Boolean))
  ;[0.15 0.15 0.15 0.5] Remove from pool
  (Utilities|Array|RemoveItem (Variables|Default|GetObjectsInUse) Target)
  (if Forced
    (Default|CallERemoveTarget)))

(event Custom|Init
  (params (WeaponStats :type S%20Weapon%20Upgrades%20Structure) (NewParam :type S%20Player%20Data%20Structure))
  (bind (_playerid _currentscore _currency _positionlastround _selectedcharacter _upgrades) (Utilities|Struct|BreakS_PlayerData NewParam))
  ;[0.15 0.15 0.15 0.5] Event begin play
  (Variables|Default|SetPlayer%20ID _playerid)
  (Variables|Default|SetWeapon%20Stats (.WeaponStats (Utilities|Struct|BreakS_PlayerUpgrades _upgrades)))
  (if (not (== (Variables|Default|GetPoolActorClass) 0))
    (CallFunction|InitPool)))

(fn FGetPooledActor
  (for _array_element (Variables|Default|GetObjectPool)
    (if (not (Variables|/Game/VFX/DemoBlueprints/Projectiles/BP_VFXProjectile.BP_VFXProjectile_C|GetIsInUse _array_element))
      (Utilities|Array|Add (Variables|Default|GetObjectsInUse) _array_element)
      (return true _array_element)))
  (return false 0))

(fn FGetOldestActorinUse
  (bind _objectsinuse (Variables|Default|GetObjectsInUse))
  (bind _output (Utilities|Array|Get(acopy) _objectsinuse))
  (Utilities|IsValid _output
    (:Is%20Valid
      (if (Utilities|Array|IsValidIndex _objectsinuse)
        (return _output true)
        (else
          _)))
    (:Is%20Not%20Valid
      _))
  (return 0 false))

(fn FRemovefromActiveList
  (params (Item :type BP%20VFX%20Projectile%20Object%20Reference%20%28by%20ref%29))
  (bind _objectsinuse (Variables|Default|GetObjectsInUse))
  (Utilities|IsValid Item
    (:Is%20Valid
      (if (Utilities|Array|ContainsItem _objectsinuse Item)
        (Utilities|Array|RemoveItem _objectsinuse Item))
      (Default|DisableActor Item))))

(fn FGetSpecificActorfromPool
  (params (ItemToFind :type BP%20VFX%20Projectile%20Object%20Reference))
  (bind _objectpool (Variables|Default|GetObjectPool))
  (if (Utilities|Array|ContainsItem _objectpool ItemToFind)
    (Utilities|Array|Add (Variables|Default|GetObjectsInUse) (Utilities|Array|Get(acopy) _objectpool (Utilities|Array|FindItem _objectpool ItemToFind)))
    (return ItemToFind true)
    (else
      (return 0 false))))