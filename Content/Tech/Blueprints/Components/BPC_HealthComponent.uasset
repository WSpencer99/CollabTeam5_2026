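; Health component that binds to its owner's any-damage event to track health and death.
; Damage handling treats negative values as healing, clamps health, broadcasts updates, fires death at zero and rumbles player controllers.
; An invincibility flag blocks damage, but the i-frame function called after each hit is empty, its timer logic disconnected.
; A separate setter sets health directly, optionally capped at max, and broadcasts the change.
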(event Custom|Death
  (Variables|Default|SetisDead true)
  (Default|CallEonDeath))

(event Custom|ExitIFrame
  (Variables|Default|SetisInvincible false))

(event EventBeginPlay
  (EventDispatchers|BindEventtoOnTakeAnyDamage (Components|GetOwner) (EventDispatchers|CreateEvent :!event FCalculateDamage)))

(fn FCalculateDamage
  (params (DamagedActor :type Actor%20Object%20Reference) (Damage :type Float%20%28single-precision%29) (DamageType :type Damage%20Type%20Object%20Reference) (InstigatedBy :type Controller%20Object%20Reference) (DamageCauser :type Actor%20Object%20Reference))
  (bind _maxhealth (Variables|Default|GetMaxHealth))
  (LocalVariables|SetL_PreviousHealth (Variables|Default|GetCurrentHealth))
  (if (Variables|Default|GetisInvincible)
    (Development|PrintString "Invincible")
    (else
      (if (< Damage 0.0)
        (if (>= (+ (* Damage -1.0) (Variables|Default|GetCurrentHealth)) _maxhealth)
          (Variables|Default|SetCurrentHealth _maxhealth)
          (else
            (Variables|Default|SetCurrentHealth (+ (* Damage -1.0) (Variables|Default|GetCurrentHealth)))))
        (elif (<= (+ (* Damage -1.0) (Variables|Default|GetCurrentHealth)) 0.0)
          (Development|PrintString "Dead")
          (Variables|Default|SetCurrentHealth 0.0)
          (CallFunction|Death)
          (else
            (Variables|Default|SetCurrentHealth (+ (* Damage -1.0) (Variables|Default|GetCurrentHealth))))))
      (Default|CallEUpdateHealth (Variables|Default|GetCurrentHealth) (LocalVariables|GetL_PreviousHealth))
      (CallFunction|FEnterIFrame true (Variables|Default|GetICooldown))
      ;[0.15 0.15 0.15 0.5] Controller Rumble
      (bind _ascontroller (Utilities|Casting|CastToController (Components|GetOwner DamagedActor)))
      (bind _asplayer_controller (Utilities|Casting|CastToPlayerController _ascontroller))
      (Game|Feedback|ClientPlayForceFeedback _asplayer_controller "/Game/Tech/Blueprints/Rumble/FF_UI.FF_UI" "" false false false))))

(fn FEnterIFrame
  (params (isInvincible :type Boolean) (Time :type Float%20%28single-precision%29)))

(fn FSetHealth
  (params (Clamped? :type Boolean) (Health :type Float%20%28double-precision%29))
  (bind _maxhealth (Variables|Default|GetMaxHealth))
  (LocalVariables|SetL_PreviousHealth (Variables|Default|GetCurrentHealth))
  (if Clamped?
    (if (> Health _maxhealth)
      (Variables|Default|SetCurrentHealth _maxhealth)
      (else
        (Variables|Default|SetCurrentHealth Health)))
    (Default|CallEUpdateHealth (Variables|Default|GetCurrentHealth) (LocalVariables|GetL_PreviousHealth))
    (else
      (Variables|Default|SetCurrentHealth Health)
      (Default|CallEUpdateHealth (Variables|Default|GetCurrentHealth) (LocalVariables|GetL_PreviousHealth)))))