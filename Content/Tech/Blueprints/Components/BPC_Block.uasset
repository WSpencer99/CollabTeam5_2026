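; Block ability component that spawns a timed BP_Shield attached to its owner, with a cooldown between uses.
; TriggerBlock acts only when no shield exists, either printing the remaining cooldown or spawning the shield and starting the cooldown timer.
; EStartBlock fires on spawn, and ResetShield clears the cooldown and fires EResetBlock.
; An unconnected branch that would spawn and attach a BP_Domain never runs.
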(event Custom|TriggerBlock
  (bind _returnvalue (Components|GetOwner))
  (Utilities|IsValid (Variables|Default|GetShieldActor)
    (:Is%20Not%20Valid
      (if (Variables|Default|GetCooldown)
        (Development|PrintString (Utilities|String|ToString(Text) (Utilities|Text|FormatText "ShieldCooldown: {TimeLeft} Seconds" (Math|Float|Truncate (Utilities|Time|GetTimerRemainingTimebyHandle (Variables|Default|GetCooldownTimer))))))
        (else
          (Variables|Default|SetCooldown true)
          (bind _returnvalue_2 (Game|SpawnActorfromClass "/Game/Tech/Blueprints/Assets/BP_Shield.BP_Shield_C" (Math|Transform|MakeTransform "0, 0, 0" "0, 0, 0" "1.000000,1.000000,1.000000") "Undefined" "MultiplyWithRoot" _returnvalue (Variables|Default|GetShieldDuration) 0))
          (bind _output_get (Variables|Default|SetShieldActor _returnvalue_2))
          (Transformation|AttachComponentToComponent _output_get (Variables|/Script/Engine.Actor|GetRootComponent _returnvalue) "None" "SnapToTarget" "KeepWorld" "KeepWorld" true)
          (Default|CallEStartBlock)
          (bind _returnvalue_3 (Utilities|Time|SetTimerbyEvent (EventDispatchers|CreateEvent :!event Custom|ResetShield) (Variables|Default|GetShieldCooldown)))
          (Variables|Default|SetCooldownTimer _returnvalue_3))))))

(event Custom|ResetShield
  (Variables|Default|SetCooldown false)
  (Default|CallEResetBlock))