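; BPC_TicketSystem is a component that tallies tickets earned during play.
; The EnemyKilled event adds a caller-supplied amount to TicketsCollected.
; EndOfRoundTickets adds a flat round bonus, plus an extra catch-up bonus when IsPlayerPositionLast is true.
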(event Custom|EnemyKilled
  (params (TicketsToAdd :type Integer))
  (Variables|Default|SetTicketsCollected (+ TicketsToAdd (Variables|Default|GetTicketsCollected))))

(event Custom|EndOfRoundTickets
  (Variables|Default|SetTicketsCollected (+ (Variables|Default|GetTicketsCollected) 50))
  (if (Variables|Default|GetIsPlayerPositionLast)
    (Variables|Default|SetTicketsCollected (+ (Variables|Default|GetTicketsCollected) 25))))