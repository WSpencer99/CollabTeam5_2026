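; Round manager for a multiplayer elimination match, running from intro to results level.
; It freezes character input during the HUD intro, then runs a countdown whose expiry triggers sudden death, setting health to one and moving the cage.
; Character deaths assign finish positions in reverse order; one survivor left triggers a time-dilated, music-fading transition.
; Finish positions are saved to the GameInstance, with last place earning extra currency, before L_Results opens.
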(event Custom|UpdateRoundStats
  (Default|RoundEnd (Variables|Default|GetHUD))
  ;[0.15 0.15 0.15 0.5] Lerp Audio Out
  (Class|BPIGameInstance|IUpdateBGMVolume(Message) (Variables|Default|GetGameInstance) false 4.0)
  (bind _newtrack_0 (Timeline|Timeline PlayFromStart)
    (:Update
      (Utilities|Time|SetGlobalTimeDilation _newtrack_0))
    (:NewTrack_1
      (bind _returnvalue (UserInterface|CreateWidget "/Game/UI/Transitions/WBP_TransitionScreen.WBP_TransitionScreen_C" 0 2.0 false true "/Game/UI/Transitions/Images/Star_Transition.Star_Transition"))
      (UserInterface|Viewport|AddtoViewport _returnvalue 1000))))

(event Custom|StartGameplay
  (Default|IToggleInput (Variables|Default|GetCharacters) true)
  (bind _returnvalue (Utilities|Time|SetTimerbyEvent (delegate Custom|EndRound) 1.0 true))
  (Variables|Default|SetRoundTimeTimerHandle _returnvalue)
  (bind _returnvalue_2 (UserInterface|CreateWidget "/Game/Tech/UI/Pause/WBP_Pause.WBP_Pause_C"))
  (bind _output_get (Variables|Default|SetPauseWidget _returnvalue_2))
  (Default|ToggleShow _output_get false)
  (UserInterface|Viewport|AddtoViewport _output_get 10)
  (for (_ _array_index) (Variables|Default|GetPlayer%20Data)
    (Class|BPIController|ISetPauseWidgetRef(Message) (Game|GetPlayerController _array_index) (Variables|Default|GetPauseWidget))))

(event Custom|End
  (bind _gameinstance (Variables|Default|GetGameInstance))
  (bind _playerfinishpositions (Variables|Default|GetPlayerFinishPositions))
  (Utilities|Time|SetGlobalTimeDilation 1.0)
  (Class|BPIGameInstance|IUpdateCurrentRoundsStats(Message) _gameinstance _playerfinishpositions)
  (bind (_keypin _valuepin) (Utilities|Map|ForEachLoop(Map) _playerfinishpositions)
    (:then
      (Class|BPIGameInstance|IAddCurrency(Message) _gameinstance (Math|Integer|SelectInt 75 50 (== _valuepin (Variables|Default|GetnumOfPlayer))) _keypin))
    (:CompletedPin
      (Game|OpenLevel(byObjectReference) "/Game/Tech/UI/Transition/Results/L_Results.L_Results"))))

(event Custom|EndRound
  (bind _result (Math|Float|DecrementFloat (Variables|Default|GetCurrentTimeRemaning))
    (:%20%20
      (Default|CallEonTimeUpdated _result)
      (if (<= _result 0.0)
        (Utilities|Time|ClearandInvalidateTimerbyHandle (Variables|Default|GetRoundTimeTimerHandle))
        (CallFunction|RoundEnd true)))))

(event EventBeginPlay
  (bind _output_get (Variables|Default|SetGameInstance (Game|GetGameInstance)))
  (Class|BPIGameInstance|IUpdateBGM(Message) _output_get "NewEnumerator1")
  (Class|BPIGameInstance|IUpdateBGM(Message) (Variables|Default|GetGameInstance) "NewEnumerator2")
  (bind _outactors (Actor|GetAllActorsOfClass "/Game/Tech/Blueprints/Player/BP_BaseCharacter.BP_BaseCharacter_C"))
  (Variables|Default|SetCharacters _outactors)
  (EventDispatchers|BindEventtoEDeath _outactors (EventDispatchers|CreateEvent :!event CheckRoundState))
  (Default|IToggleInput _outactors false)
  (Utilities|FlowControl|Sequence
    (:then_0
      (bind _playerdata (Class|BPIGameInstance|IGetPlayerData(Message) (Variables|Default|GetGameInstance)))
      (bind _output_get_2 (Variables|Default|SetPlayer%20Data _playerdata))
      (for _array_element _output_get_2
        (Utilities|Map|Add (Variables|Default|GetPlayerFinishPositions) (.PlayerID (Utilities|Struct|BreakS_PlayerData _array_element)) 1))
      (Variables|Default|SetnumOfPlayer (Utilities|Array|Length _output_get_2)))
    (:then_1
      (bind _returnvalue (UserInterface|CreateWidget "/Game/Tech/UI/WBP_RoundStart.WBP_RoundStart_C"))
      (bind _output_get_3 (Variables|Default|SetHUD _returnvalue))
      (UserInterface|Viewport|AddtoViewport _output_get_3 0)
      (EventDispatchers|BindEventtoEIntroComplete (Variables|Default|GetHUD) (EventDispatchers|CreateEvent :!event Custom|StartGameplay))
      (EventDispatchers|BindEventtoEEnd (Variables|Default|GetHUD) (EventDispatchers|CreateEvent :!event Custom|End))
      (Default|PlayIntro (Variables|Default|GetHUD))
      (bind _returnvalue_2 (UserInterface|CreateWidget "/Game/Tech/UI/WBP_GameHUD.WBP_GameHUD_C" (Game|GetPlayerController 0)))
      (Default|Init _returnvalue_2 self)
      (UserInterface|Viewport|AddtoViewport _returnvalue_2 0)
      (bind _roundtime (Class|BPIGameInstance|IGetRoundStats(Message) (Variables|Default|GetGameInstance)))
      (bind _output_get_4 (Variables|Default|SetRoundTime _roundtime))
      (Variables|Default|SetCurrentTimeRemaning _output_get_4)
      (Default|CallEonTimeUpdated (Variables|Default|GetCurrentTimeRemaning)))))

(fn ConstructionScript)

(fn CheckRoundState
  (params (PlayerController :type Player%20Controller%20Object%20Reference))
  (bind _numofplayer (Variables|Default|GetnumOfPlayer))
  (bind _playersdead (Variables|Default|GetplayersDead))
  (bind _result (Math|Integer|IncrementInt _playersdead)
    (:%20%20
      (Utilities|Map|Add (Variables|Default|GetPlayerFinishPositions) (Class|GameplayStatics|GetPlayerControllerID PlayerController) (+ (- _numofplayer _result) 1))
      (Development|PrintString (Utilities|String|Append (Utilities|GetDisplayName PlayerController) " // " (Utilities|String|ToString(Integer) (+ (- _numofplayer _result) 1))))
      (if (== (- _numofplayer 1) _playersdead)
        (CallFunction|RoundEnd false)))))

(fn RoundEnd
  (params (SuddenDeath :type Boolean))
  (if SuddenDeath
    (Default|CallSuddenDeath)
    (Class|BPIGameInstance|IUpdateBGM(Message) (Variables|Default|GetGameInstance) "NewEnumerator5")
    (bind _outactors (Actor|GetAllActorsOfClass "/Game/Tech/Blueprints/Player/BP_BaseCharacter.BP_BaseCharacter_C"))
    (for _array_element _outactors
      (Default|FSetHealth (Variables|/Game/Tech/Blueprints/Player/BP_BaseCharacter.BP_BaseCharacter_C|GetBPC_HealthComponent _array_element) false 1.0))
    (bind _returnvalue (Actor|GetActorOfClass "/Game/Tech/Blueprints/Hazards/BP_Cage.BP_Cage_C"))
    (Default|Move _returnvalue)
    (else
      (CallFunction|UpdateRoundStats))))