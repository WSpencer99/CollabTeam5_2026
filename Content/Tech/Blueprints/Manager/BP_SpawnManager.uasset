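; Manager that sets up a local multiplayer match: it loads a level layout, then spawns players and the game manager.
; BeginPlay reads the player count from GameInstance data and binds to the level-shown event of the layout selector's load.
; Init creates controllers, spawns each player's selected character at a PlayerStart, possesses it and binds its death event.
; It also points the first controller's view at a shared CameraActor and spawns BP_GameManager.
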(event Custom|Init
  (CallFunction|FAssignPlayerStarts)
  (CallFunction|FSpawnPlayerControllers)
  (CallFunction|FSpawnPlayers)
  (bind _returnvalue (Actor|GetActorOfClass "/Script/Engine.CameraActor"))
  (Game|Player|SetViewTargetwithBlend (Game|GetPlayerController 0) _returnvalue 0.0 "VTBlend_Linear" 0.0 false)
  (bind _returnvalue_2 (Game|SpawnActorfromClass "/Game/Tech/Blueprints/Manager/BP_GameManager.BP_GameManager_C" (Math|Transform|MakeTransform "0, 0, 0" "0, 0, 0" "1.000000,1.000000,1.000000") "Undefined" "MultiplyWithRoot" 0 0))
  (Variables|Default|SetGameManager _returnvalue_2))

(event EventBeginPlay
  (Variables|Default|SetPlayerAmount (CallFunction|FGetPlayerCount))
  (bind _returnvalue (Actor|GetActorOfClass "/Game/Tech/Blueprints/Manager/BP_LevelLayoutSelector.BP_LevelLayoutSelector_C"))
  (bind _returnvalue_2 (Default|FLoadLevel _returnvalue))
  (EventDispatchers|BindEventtoOnLevelShown _returnvalue_2 (EventDispatchers|CreateEvent :!event Custom|Init)))

(fn ConstructionScript)

(fn FGetPlayerCount
  (bind _playerdata (Class|BPIGameInstance|IGetPlayerData(Message) (Game|GetGameInstance)))
  (return (Utilities|Array|Length _playerdata)))

(fn FAssignPlayerStarts
  (bind _outactors (Actor|GetAllActorsOfClass "/Script/Engine.PlayerStart"))
  (Variables|Default|SetPlayerStarts _outactors))

(fn FSpawnPlayerControllers
  (for _index (range 1 (Variables|Default|GetPlayerAmount))
    (Class|GameplayStatics|CreatePlayer -1)))

(fn FSpawnPlayers
  (for _index (range 0 (- (Variables|Default|GetPlayerAmount) 1))
    (CallFunction|FPossessPlayer _index (Utilities|Array|Get(acopy) (Variables|Default|GetPlayerStarts) _index))))

(fn FPossessPlayer
  (params (ID :type Integer) (PlayerStart :type Player%20Start%20Object%20Reference))
  (bind _returnvalue (Transformation|GetActorTransform PlayerStart))
  (bind _returnvalue_2 (Game|GetPlayerController ID))
  (bind _playerdata (Class|BPIGameInstance|IGetPlayerData(Message) (Game|GetGameInstance)))
  ;[0.15 0.15 0.15 0.5] Should pass through gameplay data here via structs
  (bind _returnvalue_3 (Game|SpawnActorfromClass (.SelectedCharacter (Utilities|Struct|BreakS_PlayerData (Utilities|Array|Get(acopy) _playerdata ID))) (Math|Transform|MakeTransform (.location _returnvalue) (.rotation _returnvalue) "1.000000,1.000000,1.000000") "AlwaysSpawn" "MultiplyWithRoot" 0 0))
  (Pawn|Possess _returnvalue_2 _returnvalue_3)
  (Default|SetControllerRef _returnvalue_3 _returnvalue_2)
  (EventDispatchers|BindEventtoEDeath _returnvalue_3 (EventDispatchers|CreateEvent (Variables|Default|GetGameManager) :!event CheckRoundState)))