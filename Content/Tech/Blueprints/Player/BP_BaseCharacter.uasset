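; Base player character for a side-on platform shooter, with per-player stats, material and HUD slate set from GameInstance data once its controller is assigned.
; Movement layers wall jumps, coyote time, jump buffering, fast fall and dash; the arm aims by stick, falling back to movement direction.
; Firing draws from a pooled-projectile component, recycling the oldest when exhausted, with spread, cooldown and auto-reload.
; Health-component death spawns an effect and destroys the actor.
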(event EonDeath(BPC_HealthComponent)
  ;[1 0 0 0.5] Health Events
  (CallFunction|Death))

(event Custom|Death
  ;[0.15 0.15 0.15 0.5] Death
  (Utilities|FlowControl|DoOnce false
    (:Completed
      (Default|CallEDeath (Variables|Default|GetPlayer%20Controller))
      (Niagara|SpawnSystematLocation "/Game/VFX/Explosions/NS_StuffingExplode.NS_StuffingExplode" (Transformation|GetActorLocation))
      (Variables|Default|SetIsDead? true)
      (Actor|DestroyActor))))

(event Custom|SetControllerRef
  (params (PlayerController :type Player%20Controller%20Object%20Reference))
  (bind _widget (Variables|Default|GetWidget))
  (bind _returnvalue (UserInterface|GetWidget _widget))
  ;[0.15 0.15 0.15 0.5] Initialise Character
  (Variables|Default|SetPlayer%20Controller PlayerController)
  (Utilities|FlowControl|Sequence
    (:then_0
      (CallFunction|FSetStats)
      ;[0.15 0.15 0.15 0.5] Init Widget Slate
      (Class|UserWidget|SetOwningPlayer _returnvalue (Game|GetPlayerController 0))
      (Class|WidgetComponent|SetOwnerPlayer _widget (Class|Widget|GetOwningLocalPlayer _returnvalue))
      (bind _aswbp_player_slate (Utilities|Casting|CastToWBP_PlayerSlate _returnvalue))
      (bind _output_get (Variables|UI|SetPlayerHUD _aswbp_player_slate))
      (Default|Init _output_get self))))

(event Input|EnhancedActionEvents|EnhancedInputActionIA_Dash
  (params (ActionValue :type Boolean) (ElapsedSeconds :type Float%20%28double-precision%29) (TriggeredSeconds :type Float%20%28double-precision%29) (InputAction :type Input%20Action%20Object%20Reference :default "/Game/Tech/Input/Game/IA_Dash.IA_Dash"))
  (:Started
    (Default|FLaunchChar (Variables|Default|GetBPC_DashComponent) (Transformation|GetWorldRotation (Variables|Default|GetAimArm)))))

(event Input|EnhancedActionEvents|EnhancedInputActionIA_Move
  (params (ActionValue :type Vector%202D%20Structure) (ElapsedSeconds :type Float%20%28double-precision%29) (TriggeredSeconds :type Float%20%28double-precision%29) (InputAction :type Input%20Action%20Object%20Reference :default "/Game/Tech/Input/Game/IA_Move.IA_Move"))
  ;[0.15 0.15 0.15 0.5] Movement
  (:Triggered
    (CallFunction|FCharacterMove (.x ActionValue) (.y ActionValue)))
  (:Canceled
    (CallFunction|FRotation (Math|Float|SelectFloat 1.0 -1.0 (> (.y (Transformation|GetActorForwardVector)) 0.0)) 0.0 :!label _label))
  (:Completed
    (goto _label)))

(event Input|EnhancedActionEvents|EnhancedInputActionIA_Aim
  (params (ActionValue :type Vector%202D%20Structure) (ElapsedSeconds :type Float%20%28double-precision%29) (TriggeredSeconds :type Float%20%28double-precision%29) (InputAction :type Input%20Action%20Object%20Reference :default "/Game/Tech/Input/Game/IA_Aim.IA_Aim"))
  ;[0.15 0.15 0.15 0.5] Aiming -
  (:Triggered
    (Variables|Aiming|SetIsAiming true)
    (CallFunction|FRotation (.x ActionValue) (.y ActionValue)))
  (:Canceled
    (Variables|Aiming|SetIsAiming false :!label _label)
    (CallFunction|FRotation (Math|Float|SelectFloat 1.0 -1.0 (> (.y (Transformation|GetActorForwardVector)) 0.0)) 0.0))
  (:Completed
    (goto _label)))

(event EventDestroyed
  ;[1 0 0 0.5] Clear Up Projectiles
  (for _array_element (Variables|/Game/Tech/Blueprints/Components/BPC_ObjectPool.BPC_ObjectPool_C|GetObjectPool (Variables|Default|GetBPC_ObjectPool))
    (Default|Destroy _array_element)))

(event EventBeginPlay)

(event Input|KeyboardEvents|DebugKeyTab
  (params (Key :type Key%20Structure :default "None") (ActionValue :type Input%20Action%20Value%20Structure))
  ;[1 0 0 0.5] Debug HUD
  (:Pressed
    (bind _isa (Utilities|FlowControl|FlipFlop)
      (:A
        _)
      (:B
        _))
    (Rendering|SetVisibility (Variables|Default|GetWidget) _isa false)
    (bind _foundwidgets (Widget|GetAllWidgetsOfClass "/Game/Tech/UI/WBP_HealthBar.WBP_HealthBar_C" false))
    (for _array_element _foundwidgets
      (Development|PrintString (Utilities|GetDisplayName _array_element)))))

(event Input|KeyboardEvents|DebugKey1
  (params (Key :type Key%20Structure :default "None") (ActionValue :type Input%20Action%20Value%20Structure))
  ;[1 0 0 0.5] Health Events
  (:Pressed
    (Game|Damage|ApplyDamage self 1e+01 0 0)))

(event Custom|CancelFastFall
  ;[0.15 0.15 0.15 0.5] Fast Falling
  (Variables|/Script/Engine.CharacterMovementComponent|SetGravityScale (Variables|Character|GetCharacterMovement) 3.0)
  (Variables|Jump|SetIsFastFalling? false))

(event Custom|ResetJumpBuffer
  ;[0.15 0.15 0.15 0.5] Jump Action
  (Variables|Jump|SetIsJumpBuffering? false)
  (Utilities|Time|ClearandInvalidateTimerbyHandle (Variables|Jump|GetJumpBufferTimerHandle)))

(event Custom|ResetCoyoteTime
  ;[0.15 0.15 0.15 0.5] Coyote Time
  (Variables|Jump|SetInCoyoteTime false)
  (Development|PrintString "NotInCoyoteTime" true true "(R=1.000000,G=0.177176,B=0.000000,A=1.000000)" 5.0 "as dad a")
  (Utilities|Time|ClearandInvalidateTimerbyHandle (Variables|Jump|GetCoyoteTimeTimerHandle)))

(event Custom|BufferedJump
  ;[0.15 0.15 0.15 0.5] Buffered Jump
  (Development|PrintString "Jumppppp")
  (CallFunction|ResetJumpBuffer)
  (Variables|Jump|SetIsJumping false)
  (Character|Jump)
  (Utilities|FlowControl|DelayUntilNextTick)
  (if (not (> (Input|EnhancedActionValues|GetIA_Jump) 0))
    (Character|StopJumping)
    (CallFunction|ResetCoyoteTime)))

(event Input|EnhancedActionEvents|EnhancedInputActionIA_FastFalling
  (params (ActionValue :type Float%20%28double-precision%29) (ElapsedSeconds :type Float%20%28double-precision%29) (TriggeredSeconds :type Float%20%28double-precision%29) (InputAction :type Input%20Action%20Object%20Reference :default "/Game/Tech/Input/Game/IA_FastFalling.IA_FastFalling"))
  ;[0.15 0.15 0.15 0.5] Fast Falling
  (:Triggered
    (if (< ActionValue -0.5)
      (Variables|Jump|SetIsFastFalling? true)
      (if (AI|Components|NavMovement|IsFalling (Variables|Character|GetCharacterMovement))
        (Variables|/Script/Engine.CharacterMovementComponent|SetGravityScale (Variables|Character|GetCharacterMovement) 7.0)
        (else
          (Variables|/Script/Engine.CharacterMovementComponent|SetGravityScale (Variables|Character|GetCharacterMovement) 3.0)
          (Variables|Jump|SetIsFastFalling? false)))
      (else
        (CallFunction|CancelFastFall :!label _label))))
  (:Canceled
    (goto _label))
  (:Completed
    (goto _label)))

(event Input|EnhancedActionEvents|EnhancedInputActionIA_Jump
  (params (ActionValue :type Boolean) (ElapsedSeconds :type Float%20%28double-precision%29) (TriggeredSeconds :type Float%20%28double-precision%29) (InputAction :type Input%20Action%20Object%20Reference :default "/Game/Tech/Input/Game/IA_Jump.IA_Jump"))
  (bind _returnvalue (Transformation|GetActorRotation))
  ;[0.15 0.15 0.15 0.5] Jump Action
  (:Started
    (if (Variables|Jump|GetWallJump?)
      (Character|LaunchCharacter (+ (* (Transformation|GetActorForwardVector) (Variables|Jump|GetWallJumpForce)) "0.000000,0.000000,1000.000000") true true)
      (Transformation|SetActorRotation (Math|Rotator|MakeRotator (.roll _returnvalue) (.pitch _returnvalue) (+ (.yaw _returnvalue) 1.8e+02)))
      (elif (Character|CanJump)
        (Variables|Jump|SetIsJumping true)
        (Character|Jump)
        (else
          (Utilities|Time|ClearandInvalidateTimerbyHandle (Variables|Jump|GetJumpBufferTimerHandle))
          (Variables|Jump|SetIsJumpBuffering? true)
          (bind _returnvalue_2 (Utilities|Time|SetTimerbyEvent (delegate Custom|ResetJumpBuffer) (Variables|Jump|GetJumpBufferTimer)))
          (Variables|Jump|SetJumpBufferTimerHandle _returnvalue_2)))))
  (:Canceled
    (Character|StopJumping :!label _label)
    (CallFunction|ResetCoyoteTime))
  (:Completed
    (goto _label)))

(event EventTick
  (params (DeltaSeconds :type Float%20%28single-precision%29))
  (bind _capsulecomponent (Variables|Collision|GetCapsuleComponent))
  (bind _charactermovement (Variables|Character|GetCharacterMovement))
  (bind _returnvalue (Transformation|GetWorldLocation _capsulecomponent))
  ;[1 0 0 0.5] Wall Jump
  ;;[1 0 0 0.5] Event Tick Just Here for Testing RN
  (if (AI|Components|NavMovement|IsFalling (Variables|Character|GetCharacterMovement))
    (bind _returnvalue_2 (Collision|LineTraceByChannel _returnvalue (+ _returnvalue (* (Math|Vector|GetForwardVector _capsulecomponent) (Variables|Jump|GetWallCheckDistance))) "TraceTypeQuery3" false 0 "None"))
    (if _returnvalue_2
      (Variables|Jump|SetWallJump? true)
      (Variables|/Script/Engine.MovementComponent|SetVelocity _charactermovement (Math|Interpolation|VInterptoConstant (Variables|/Script/Engine.MovementComponent|GetVelocity _charactermovement) "0, 0, 0" (Utilities|Time|GetWorldDeltaSeconds) 3e+03))
      (else
        (Variables|Jump|SetWallJump? false :!label _label)))
    (else
      (goto _label))))

(event EventOnMovementModeChanged
  (params (PrevMovementMode :type EMovementMode%20Enum :default "MOVE_None") (NewMovementMode :type EMovementMode%20Enum :default "MOVE_None") (PrevCustomMode :type Byte :default 0) (NewCustomMode :type Byte :default 0))
  ;[0.15 0.15 0.15 0.5] Coyote Time
  (switch Utilities|FlowControl|Switch|SwitchonEMovementMode PrevMovementMode
    (:MOVE_Walking
      (Variables|/Script/Engine.CharacterMovementComponent|SetFallingLateralFriction (Variables|Character|GetCharacterMovement) 5.901367)
      (switch Utilities|FlowControl|Switch|SwitchonEMovementMode NewMovementMode
        (:MOVE_Falling
          (Utilities|Time|ClearandInvalidateTimerbyHandle (Variables|Jump|GetCoyoteTimeTimerHandle))
          (Variables|Jump|SetInCoyoteTime true)
          (bind _returnvalue (Utilities|Time|SetTimerbyEvent (delegate Custom|ResetCoyoteTime) (Variables|Jump|GetCoyoteTime)))
          (Variables|Jump|SetCoyoteTimeTimerHandle _returnvalue)
          (Development|PrintString "CoyoteTime" true true "(R=1.000000,G=0.177176,B=0.000000,A=1.000000)" 5.0 "as dad a"))))))

(event EventOnLanded
  (params (Hit :type Hit%20Result%20Structure%20%28by%20ref%29))
  ;[0.15 0.15 0.15 0.5] Event On Landed
  (Utilities|FlowControl|Sequence
    (:then_0
      ;[0.15 0.15 0.15 0.5] Reset Fast Fall
      (CallFunction|CancelFastFall))
    (:then_1
      ;[0.15 0.15 0.15 0.5] Jump Buffering
      (if (Variables|Jump|GetIsJumpBuffering?)
        (Utilities|FlowControl|DelayUntilNextTick)
        (CallFunction|BufferedJump)
        (else
          (Variables|Jump|SetIsJumping false))))))

(event Custom|CompleteReload
  (bind _output_get (Variables|Default|SetCurrentAmmo (Variables|Default|GetMaxAmmo)))
  (Default|CallEUpdateAmmo _output_get)
  (Variables|Default|SetIsReloading? false))

(event Custom|StartReload
  (bind _reloadtime (Variables|Default|GetReloadTime))
  (Variables|Default|SetIsReloading? true)
  (Default|CallEReload _reloadtime)
  (Variables|Default|SetCurrentAmmo 0)
  (Utilities|Time|SetTimerbyEvent (EventDispatchers|CreateEvent :!event Custom|CompleteReload) _reloadtime))

(event Input|EnhancedActionEvents|EnhancedInputActionIA_Reload
  (params (ActionValue :type Boolean) (ElapsedSeconds :type Float%20%28double-precision%29) (TriggeredSeconds :type Float%20%28double-precision%29) (InputAction :type Input%20Action%20Object%20Reference :default "/Game/Tech/Input/Game/IA_Reload.IA_Reload"))
  (:Started
    (if (not (or (Variables|Default|GetIsReloading?) (>= (Variables|Default|GetCurrentAmmo) (Variables|Default|GetMaxAmmo))))
      (CallFunction|StartReload))))

(event Input|EnhancedActionEvents|EnhancedInputActionIA_Fire
  (params (ActionValue :type Boolean) (ElapsedSeconds :type Float%20%28double-precision%29) (TriggeredSeconds :type Float%20%28double-precision%29) (InputAction :type Input%20Action%20Object%20Reference :default "/Game/Tech/Input/Game/IA_Fire.IA_Fire"))
  ;[1 0 0 0.5] ObjectPooling spawn system
  (if (not (Variables|Default|GetWeaponInCooldown))
    (CallFunction|FFireWeapon)))

(fn ConstructionScript)

(fn CanJumpInternal
  (bind _returnvalue (|CallParentFunction))
  (return (or (and _returnvalue (Variables|Jump|GetAllowJump)) (Variables|Jump|GetInCoyoteTime))))

(fn FRotation
  (params (X :type Float%20%28double-precision%29) (Y :type Float%20%28double-precision%29))
  (bind _returnvalue (* Y -1.0))
  (bind _returnvalue_2 (Math|Trig|Atan2(Radians) _returnvalue X))
  (bind _returnvalue_3 (Math|Trig|RadiansToDegrees _returnvalue_2))
  (if (> (Math|Float|Absolute(Float) (Math|Vector2D|Vector2DLength (Math|Vector2D|MakeVector2D X Y))) (Variables|Aiming|GetAimDeadzone))
    (Transformation|SetWorldRotation (Variables|Default|GetAimArm) (Math|Rotator|MakeRotator 0.0 _returnvalue_3 9e+01) false false)
    (if (> (Math|Float|Absolute(Float) _returnvalue_3) 9e+01)
      _)))

(fn FJumpCheck
  (if (and (Character|CanJump) (Variables|Jump|GetAllowJump))
    (return true)
    (elif (Variables|Jump|GetInCoyoteTime)
      (CallFunction|ResetCoyoteTime)
      (return true)
      (else
        (return false)))))

(fn FCharacterMove
  (params (X :type Float%20%28double-precision%29) (Y :type Float%20%28double-precision%29))
  (Pawn|Input|AddMovementInput (Math|Vector|MakeVector 0.0 X 0.0) 1.0 false)
  ;[0.15 0.15 0.15 0.5] Perform Aiming based on movement if Aim input is not being held
  (if (not (Variables|Aiming|GetIsAiming))
    (CallFunction|FRotation X (* Y -1.0))))

(fn FireProjectile
  (bind _projectile_spawn_point (Variables|Default|GetProjectile%20Spawn%20Point))
  (bind _returnvalue (Transformation|GetWorldTransform _projectile_spawn_point))
  (bind _projectile (Default|GetProjectile (Variables|Default|GetpoolManager)))
  (Utilities|IsValid _projectile
    (:Is%20Valid
      (Transformation|SetActorTransform _projectile (Math|Transform|MakeTransform (.location _returnvalue) (.rotation _returnvalue) "1.000000,1.000000,1.000000"))
      (Actor|SetOwner _projectile self)
      (Default|Activate _projectile)
      (Default|StartDeleteTimer _projectile))
    (:Is%20Not%20Valid
      (Development|PrintString "Object Pool Actor Not Found" true true "(R=1.000000,G=0.066860,B=0.000000,A=1.000000)" 1e+01))))

(fn FSetStats
  (bind _playerdata (Class|BPIGameInstance|IGetPlayerData(Message) (Game|GetGameInstance)))
  (Utilities|FlowControl|Sequence
    (:then_0
      (CallFunction|FSetWeaponStats (.WeaponStats (Utilities|Struct|BreakS_PlayerUpgrades (.Upgrades (Utilities|Struct|BreakS_PlayerData (Utilities|Array|Get(acopy) _playerdata (Class|GameplayStatics|GetPlayerControllerID (Variables|Default|GetPlayer%20Controller)))))))))
    (:then_1
      (CallFunction|FSetPlayerStats (.PlayerStats (Utilities|Struct|BreakS_PlayerUpgrades (.Upgrades (Utilities|Struct|BreakS_PlayerData (Utilities|Array|Get(acopy) _playerdata (Class|GameplayStatics|GetPlayerControllerID (Variables|Default|GetPlayer%20Controller)))))))))
    (:then_2
      (Rendering|Material|SetMaterial (Variables|Character|GetMesh) 0 (Utilities|Select :Index (.PlayerID (Utilities|Struct|BreakS_PlayerData (Utilities|Array|Get(acopy) _playerdata (Class|GameplayStatics|GetPlayerControllerID (Variables|Default|GetPlayer%20Controller))))) :Option%200 "/Game/Assets/Character/Test/Base_EarsAndNose_Inst.Base_EarsAndNose_Inst" :Option%201 "/Game/Assets/Character/Test/Base_EarsAndNose_Inst1.Base_EarsAndNose_Inst1" :Option%202 "/Game/Assets/Character/Test/Base_EarsAndNose_Inst3.Base_EarsAndNose_Inst3" :Option%203 "/Game/Assets/Character/Test/Base_EarsAndNose_Inst2.Base_EarsAndNose_Inst2")))))

(fn FSetWeaponStats
  (params (WeaponStats :type S%20Weapon%20Upgrades%20Structure))
  (bind (_ammocapacity _damage _projectilespeed _firerate _reloadtime _damagetype _movementtype _bulletspread) (Utilities|Struct|BreakS_WeaponUpgrades WeaponStats))
  (Default|Init (Variables|Default|GetBPC_ObjectPool) WeaponStats)
  (Variables|Default|SetFireRate _firerate)
  (Variables|Default|SetReloadTime _reloadtime)
  (bind _output_get (Variables|Default|SetMaxAmmo _ammocapacity))
  (Variables|Default|SetCurrentAmmo _output_get)
  (Variables|Default|SetBulletSpread _bulletspread))

(fn FFireWeapon
  (bind _bpc_objectpool (Variables|Default|GetBPC_ObjectPool))
  (bind _bulletspread (Variables|Default|GetBulletSpread))
  (if (not (Variables|Default|GetWeaponInCooldown))
    (if (> (Variables|Default|GetCurrentAmmo) 0)
      (bind _result (Math|Integer|DecrementInt (Variables|Default|GetCurrentAmmo))
        (:%20%20
          (Default|CallEUpdateAmmo _result)
          (bind (_issuccess _projectile) (Default|FGetPooledActor (Variables|Default|GetBPC_ObjectPool)))
          (LocalVariables|SetL_Transform (Transformation|GetWorldTransform (Variables|Default|GetProjectile%20Spawn%20Point)))
          (if _issuccess
            (bind _output_get (LocalVariables|SetL_Projectile _projectile))
            (Default|EnableActor _output_get (Math|Transform|MakeTransform (.location (LocalVariables|GetL_Transform)) (Math|Rotator|MakeRotator (.roll (.rotation (LocalVariables|GetL_Transform))) (+ (.pitch (.rotation (LocalVariables|GetL_Transform))) (Math|Random|RandomFloatinRange (* _bulletspread -1.0) _bulletspread)) (.yaw (.rotation (LocalVariables|GetL_Transform)))) (.scale (LocalVariables|GetL_Transform))) :!label _label)
            (Variables|Default|SetWeaponInCooldown true)
            (bind _returnvalue (Utilities|Time|SetTimerbyEvent (EventDispatchers|CreateEvent :!event FExitCooldown) (Variables|Default|GetFireRate)))
            (Variables|Default|SetCooldownTimer _returnvalue)
            (Development|PrintString "Shoot")
            (if (<= (Variables|Default|GetCurrentAmmo) 0)
              (CallFunction|StartReload))
            (else
              (bind (_output _found) (Default|FGetOldestActorinUse _bpc_objectpool))
              (if _found
                (bind _output_get_2 (LocalVariables|SetL_Projectile _output))
                (Default|FRemovefromActiveList _bpc_objectpool _output_get_2)
                (bind _success (Default|FGetSpecificActorfromPool _bpc_objectpool (LocalVariables|GetL_Projectile)))
                (if _success
                  (goto _label)))))))
      (elif (not (Variables|Default|GetIsReloading?))
        (CallFunction|StartReload)))))

(fn FExitCooldown
  (Variables|Default|SetWeaponInCooldown false))

(fn FSetPlayerStats
  (params (PlayerStats :type S%20Player%20Stats%20Upgrades%20Structure))
  (bind (_health _movementspeed _jumpheight _jumpgravity _dashstrength _dashcooldown) (Utilities|Struct|BreakS_PlayerStatsUpgrades PlayerStats))
  (bind _bpc_healthcomponent (Variables|Default|GetBPC_HealthComponent))
  (bind _charactermovement (Variables|Character|GetCharacterMovement))
  (bind _bpc_dashcomponent (Variables|Default|GetBPC_DashComponent))
  (Variables|/Game/Tech/Blueprints/Components/BPC_HealthComponent.BPC_HealthComponent_C|SetCurrentHealth _bpc_healthcomponent _health)
  (Variables|/Game/Tech/Blueprints/Components/BPC_HealthComponent.BPC_HealthComponent_C|SetMaxHealth _bpc_healthcomponent _health)
  (Variables|/Script/Engine.CharacterMovementComponent|SetJumpZVelocity _charactermovement _jumpheight)
  (bind _output_get (Variables|/Script/Engine.CharacterMovementComponent|SetGravityScale _charactermovement _jumpgravity))
  (Variables|Default|SetDefaultGravity _output_get)
  (Variables|/Script/Engine.CharacterMovementComponent|SetMaxWalkSpeed _charactermovement _movementspeed)
  (Variables|/Game/Tech/Blueprints/Components/BPC_DashComponent.BPC_DashComponent_C|SetDashStrength _bpc_dashcomponent _dashstrength)
  (Variables|/Game/Tech/Blueprints/Components/BPC_DashComponent.BPC_DashComponent_C|SetDashCooldown _bpc_dashcomponent _dashcooldown))